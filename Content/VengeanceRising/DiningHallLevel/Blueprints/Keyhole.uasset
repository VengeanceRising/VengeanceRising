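; Keyhole is an interactable in the Dining Hall level that opens the magic fireplace puzzle when the player carries the key.
; Interact searches the game instance's Inventory for an item with the Tifanny_fbx mesh, so the key is identified by mesh.
; With the key, it calls Move on the first BP_Magic_Fireplace found in the world; otherwise it prints a needs-a-key message.
; GetDetails, Talk and Thinking are empty stubs.
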(event EventBeginPlay)

(event EventActorBeginOverlap
  (params (OtherActor :type Actor%20Object%20Reference)))

(event EventTick
  (params (DeltaSeconds :type Float%20%28single-precision%29)))

(fn ConstructionScript)

(fn GetDetails
  (return ""))

(fn Interact
  (bind _asvengeance_rising_game_instance (Utilities|Casting|CastToVengeanceRisingGameInstance (Game|GetGameInstance))
    (:then
      (bind _array_element (Utilities|Array|ForEachLoopwithBreak (Variables|/Game/VengeanceRising/VengeanceRisingGameInstance.VengeanceRisingGameInstance_C|GetInventory _asvengeance_rising_game_instance) :!label _label)
        (:LoopBody
          (if (== (.Mesh (Utilities|Struct|BreakBPS_Item _array_element)) "/Game/VengeanceRising/Stefan/Meshes/Keys/Tifanny_fbx.Tifanny_fbx")
            (Variables|Default|SetHasKey true)
            (goto _label Break)))
        (:Completed
          (if (Variables|Default|GetHasKey)
            (bind _outactors (Actor|GetAllActorsOfClass "/Game/VengeanceRising/DiningHallLevel/Blueprints/BP_Magic_Fireplace.BP_Magic_Fireplace_C"))
            (bind _array_element_2 (Utilities|Array|ForEachLoopwithBreak _outactors :!label _label_2)
              (:LoopBody
                (Default|Move _array_element_2)
                (goto _label_2 Break))
              (:Completed
                _))
            (else
              (Development|PrintString "Seems like I need a key for that.")))
          (return 0))))
    (:CastFailed
      (return 0))))

(fn Talk
  (params (Index :type Integer))
  (return false))

(fn Thinking
  (return false))