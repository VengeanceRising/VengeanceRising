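; BP_RockingChair is an interactable dining hall prop that creaks when something overlaps its Box and shows a thought subtitle when used.
; An IsPlayingSound flag with delays suppresses the creak briefly after BeginPlay and prevents retriggering while the sound plays.
; Interact passes the indexed Thoughts entry to the player's DisplaySubtitles; the other interaction functions, such as Outline and Talk, are stubs.
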(event OnComponentBeginOverlap(Box)
  (params (OtherActor :type Actor%20Object%20Reference) (OtherComp :type Primitive%20Component%20Object%20Reference) (OtherBodyIndex :type Integer) (bFromSweep :type Boolean) (SweepResult :type Hit%20Result%20Structure%20%28by%20ref%29))
  (if (not (Variables|Default|GetIsPlayingSound))
    (Variables|Default|SetIsPlayingSound true)
    (Audio|SpawnSoundatLocation "/Game/VengeanceRising/Commons/Sounds/153120__victoriarey91__chair-in-movement.153120__victoriarey91__chair-in-movement" (Transformation|GetActorLocation) "0, 0, 0" 5.0)
    (Utilities|FlowControl|Delay 1.4)
    (Variables|Default|SetIsPlayingSound false)
    (Utilities|FlowControl|DoOnce false) ; enters at Reset
  ))

(event EventBeginPlay
  (Variables|Default|SetIsPlayingSound true)
  (Utilities|FlowControl|Delay 2.0)
  (Variables|Default|SetIsPlayingSound false))

(event EventTick
  (params (DeltaSeconds :type Float%20%28single-precision%29)))

(fn ConstructionScript)

(fn ActivateOption
  (return 0))

(fn Interact
  (bind _asbp_dining_hall_player (Utilities|Casting|CastToBP_DiningHallPlayer (Game|Player|GetPlayerPawn 0))
    (:then
      (Default|DisplaySubtitles _asbp_dining_hall_player (Utilities|Array|Get(acopy) (Variables|Default|GetThoughts) (Variables|Default|GetThought%20Index))))
    (:CastFailed
      _))
  (return false "0, 0, 0" ""))

(fn NoOutline
  (return false))

(fn Outline
  (return false))

(fn Talk
  (params (Index :type Integer))
  (return false))

(fn Thinking
  (return false))