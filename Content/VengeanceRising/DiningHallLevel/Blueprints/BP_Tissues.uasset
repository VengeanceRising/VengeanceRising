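; BP_Tissues is an interactable tissues pickup in the Dining Hall level that can be highlighted, examined and collected.
; Interact offers a "Pick Up" option box, and ActivateOption adds the item to VengeanceRisingGameInstance, then destroys the actor.
; Outline and NoOutline toggle custom depth on both meshes, while Thinking displays an indexed thought as a player subtitle.
; Talk is unused and returns false, and the event graph is empty.
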(event EventBeginPlay)

(event EventActorBeginOverlap
  (params (OtherActor :type Actor%20Object%20Reference)))

(event EventTick
  (params (DeltaSeconds :type Float%20%28single-precision%29)))

(fn ConstructionScript)

(fn ActivateOption
  (bind _asvengeance_rising_game_instance (Utilities|Casting|CastToVengeanceRisingGameInstance (Game|GetGameInstance))
    (:then
      (Default|AddItem _asvengeance_rising_game_instance (Variables|Default|GetItem))
      (Actor|DestroyActor))
    (:CastFailed
      _))
  (return 0))

(fn Interact
  (return true (Variables|Default|GetSpawnOffset) "Pick Up"))

(fn NoOutline
  (Rendering|SetRenderCustomDepth (Variables|Default|GetStaticMesh) false)
  (return false))

(fn Outline
  (Rendering|SetRenderCustomDepth (Variables|Default|GetStaticMesh) true)
  (return true))

(fn Talk
  (params (Index :type Integer))
  (return false))

(fn Thinking
  (bind _asbp_dining_hall_player (Utilities|Casting|CastToBP_DiningHallPlayer (Game|Player|GetPlayerPawn 0))
    (:then
      (Default|DisplaySubtitles _asbp_dining_hall_player (Utilities|Array|Get(acopy) (Variables|Default|GetThoughts) (Variables|Default|GetThoughtIndex))))
    (:CastFailed
      _))
  (return true))