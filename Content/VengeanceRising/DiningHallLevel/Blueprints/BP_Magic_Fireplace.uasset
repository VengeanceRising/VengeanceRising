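; BP_Magic_Fireplace is a dining hall fireplace that toggles open and closed with a hidden-wall sound.
; Move flips IsOpen and plays or reverses the first MatineeActor found in the level; IsMoving resets immediately rather than when the animation ends.
; Thinking shows the current thought as a subtitle on BP_DiningHallPlayer.
; Interact, Talk and ActivateOption return empty defaults, and the event graph and its Timeline are unused.
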(event EventBeginPlay)

(event Collision|EventActorBeginOverlap
  (params (OtherActor :type Actor%20Object%20Reference)))

(event EventTick
  (params (DeltaSeconds :type Float%20%28single-precision%29)))

(fn ConstructionScript)

(fn Move
  (if (not (Variables|Default|GetIsMoving))
    (Variables|Default|SetIsMoving true)
    (Utilities|FlowControl|Sequence
      (:then_0
        (if (Variables|Default|GetIsOpen)
          (Variables|Default|SetIsOpen false)
          (bind _outactors (Actor|GetAllActorsOfClass "/Script/Engine.MatineeActor"))
          (Utilities|String|Reverse (Utilities|Array|Get(acopy) _outactors))
          (Audio|PlaySoundatLocation "/Game/VengeanceRising/Commons/Sounds/243699__ertfelda__hidden-wall-opening.243699__ertfelda__hidden-wall-opening" (Transformation|GetWorldLocation (Variables|Default|GetStaticMesh)) "0, 0, 0" 1.0)
          (else
            (Variables|Default|SetIsOpen true)
            (bind _outactors_2 (Actor|GetAllActorsOfClass "/Script/Engine.MatineeActor"))
            (Audio|Components|Audio|Play (Utilities|Array|Get(acopy) _outactors_2))
            (Audio|PlaySoundatLocation "/Game/VengeanceRising/Commons/Sounds/243699__ertfelda__hidden-wall-opening.243699__ertfelda__hidden-wall-opening" (Transformation|GetWorldLocation (Variables|Default|GetStaticMesh)) "0, 0, 0" 1.0))))
      (:then_1
        (Variables|Default|SetIsMoving false)))))

(fn ActivateOption
  (return 0))

(fn Interact
  (return false "0, 0, 0" ""))

(fn Talk
  (params (Index :type Integer))
  (return false))

(fn Thinking
  (bind _asbp_dining_hall_player (Utilities|Casting|CastToBP_DiningHallPlayer (Game|Player|GetPlayerPawn 0))
    (:then
      (Default|DisplaySubtitles _asbp_dining_hall_player (Utilities|Array|Get(acopy) (Variables|Default|GetThoughts) (Variables|Default|GetThoughtIndex))))
    (:CastFailed
      _))
  (return false))