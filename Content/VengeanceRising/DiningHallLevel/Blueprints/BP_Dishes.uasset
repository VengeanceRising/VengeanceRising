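; BP_Dishes is an interactable dishes prop for the dining hall level that gives the player a thought as a subtitle.
; Interact casts the player pawn to BP_DiningHallPlayer and displays the entry of Thoughts at ThoughtsIndex.
; Outline and NoOutline toggle custom depth rendering on its five static meshes for highlighting.
; ActivateOption, Talk and Thinking only return default values, and the event graph is inactive.
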(event EventBeginPlay)

(event EventActorBeginOverlap
  (params (OtherActor :type Actor%20Object%20Reference)))

(event EventTick
  (params (DeltaSeconds :type Float%20%28single-precision%29)))

(fn ConstructionScript)

(fn ActivateOption
  (return 0))

(fn Interact
  (bind _asbp_dining_hall_player (Utilities|Casting|CastToBP_DiningHallPlayer (Game|Player|GetPlayerPawn 0))
    (:then
      (Default|DisplaySubtitles _asbp_dining_hall_player (Utilities|Array|Get(acopy) (Variables|Default|GetThoughts) (Variables|Default|GetThoughts%20Index))))
    (:CastFailed
      _))
  (return false "0, 0, 0" ""))

(fn NoOutline
  (Rendering|SetRenderCustomDepth (Variables|Default|GetStaticMesh4) false)
  (return false))

(fn Outline
  (Rendering|SetRenderCustomDepth (Variables|Default|GetStaticMesh) true)
  (return true))

(fn Talk
  (params (Index :type Integer))
  (return false))

(fn Thinking
  (return false))