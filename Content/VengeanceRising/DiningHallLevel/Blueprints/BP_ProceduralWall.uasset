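; Procedural wall Blueprint for the dining hall level, built in the construction script from EndPoint and a shared Material.
; It applies the material to BaseFloor, then nested loops attach mesh tiles to it on a 400-unit local X/Y grid.
; Column count follows EndPoint's horizontal length.
; Row count multiplies EndPoint by a zero vector, so as written no tiles are added.
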(event EventBeginPlay)

(event Collision|EventActorBeginOverlap
  (params (OtherActor :type Actor%20Object%20Reference)))

(event EventTick
  (params (DeltaSeconds :type Float%20%28single-precision%29)))

(fn ConstructionScript
  (bind _endpoint (Variables|Default|GetEndPoint))
  (Rendering|Material|SetMaterial (Variables|Default|GetBaseFloor) 0 (Variables|Default|GetMaterial))
  (if (Math|Vector|NotEqual(Vector) (* (Variables|Default|GetEndPoint) "1.000000,1.000000, 0") "0, 0, 0" 0.0001)
    (for _index (range 0 (- (Math|Float|Ceil (/ (Math|Vector|VectorLength (* _endpoint "0.000000,0.000000,0.000000")) 4e+02)) 1))
      (for _index_2 (range 0 (- (Math|Float|Ceil (/ (Math|Vector|VectorLength (* _endpoint "1.000000,1.000000, 0")) 4e+02)) 1))
        (bind _returnvalue (AddComponent|AddStaticMeshComponent false))
        (Rendering|Material|SetMaterial _returnvalue 0 (Variables|Default|GetMaterial))
        (Class|SceneComponent|Attachto _returnvalue (Variables|Default|GetBaseFloor) "None" "KeepRelativeOffset" true)
        (Transformation|SetRelativeLocation _returnvalue (+ (Math|Vector|MakeVector (* _index_2 4e+02) 0.0 0.0) (Math|Vector|MakeVector 0.0 (* _index 4e+02) 0.0)) false false)))))