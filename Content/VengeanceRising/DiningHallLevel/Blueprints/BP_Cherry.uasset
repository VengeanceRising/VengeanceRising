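; BP_Cherry is a cherry pickup in the dining hall level that the player can add to the inventory.
; It implements interaction functions: GetDetails returns its Item with CanPickUp false, and Talk always returns false.
; Interact fetches the item through GetDetails, adds it to the VengeanceRising game instance, prints a confirmation and destroys the actor, without checking CanPickUp.
; The event graph and construction script are empty.
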(event EventBeginPlay)

(event EventActorBeginOverlap
  (params (OtherActor :type Actor%20Object%20Reference)))

(event EventTick
  (params (DeltaSeconds :type Float%20%28single-precision%29)))

(fn ConstructionScript)

(fn GetDetails
  (return (Variables|Default|GetItem) false))

(fn Interact
  (bind _item (Class|BPIItemPickUp|GetDetails(Message) self))
  (bind _asvengeance_rising_game_instance (Utilities|Casting|CastToVengeanceRisingGameInstance (Game|GetGameInstance))
    (:then
      (Default|AddItem _asvengeance_rising_game_instance _item)
      (Development|PrintString (Utilities|String|Append (Utilities|String|ToString(Text) (.Name (Utilities|Struct|BreakBPS_Item (Variables|Default|GetItem)))) " was put in the inventory"))
      (Actor|DestroyActor))
    (:CastFailed
      _))
  (return 1))

(fn Talk
  (params (Index :type Integer))
  (return false))