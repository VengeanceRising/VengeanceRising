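; BP_Key_Tifanny is an interactable pickup in the Dining Hall level, by its name Tifanny's key.
; Interact requests an interaction box, and ActivateOption adds the Item to the game instance, advances the checkpoint, prints a pickup message and destroys the actor.
; Thinking shows the current Thoughts entry as a subtitle through the Dining Hall player, while Talk is an empty stub returning false.
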(event EventBeginPlay)

(event EventActorBeginOverlap
  (params (OtherActor :type Actor%20Object%20Reference)))

(event EventTick
  (params (DeltaSeconds :type Float%20%28single-precision%29)))

(fn ConstructionScript)

(fn ActivateOption
  (bind _asvengeance_rising_game_instance (Utilities|Casting|CastToVengeanceRisingGameInstance (Game|GetGameInstance))
    (:then
      (Default|AddItem _asvengeance_rising_game_instance (Variables|Default|GetItem))
      (Default|NextCheckpoint _asvengeance_rising_game_instance)
      (Development|PrintString (Utilities|String|Append (Utilities|String|ToString(Text) (.Name (Utilities|Struct|BreakBPS_Item (Variables|Default|GetItem)))) " was put in the inventory"))
      (Actor|DestroyActor))
    (:CastFailed
      _))
  (return 0))

(fn Interact
  (return true "0, 0, 0" ""))

(fn Talk
  (params (Index :type Integer))
  (return false))

(fn Thinking
  (bind _asbp_dining_hall_player (Utilities|Casting|CastToBP_DiningHallPlayer (Game|Player|GetPlayerPawn 0))
    (:then
      (Default|DisplaySubtitles _asbp_dining_hall_player (Utilities|Array|Get(acopy) (Variables|Default|GetThoughts) (Variables|Default|GetThoughtIndex))))
    (:CastFailed
      _))
  (return false))