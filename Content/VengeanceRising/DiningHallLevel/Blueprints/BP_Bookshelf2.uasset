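; BP_Bookshelf2 is a bookshelf prop that optionally fills itself with books in the construction script; it has no active runtime logic.
; For each shelf height whose row option is 1, it adds static mesh books across every column, spaced by scaled book width up to that column's count.
; BookOption1 selects between two book component variants with different material slots, and BookOption2 picks which of two materials is applied.
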(event EventBeginPlay)

(event Collision|EventActorBeginOverlap
  (params (OtherActor :type Actor%20Object%20Reference)))

(event EventTick
  (params (DeltaSeconds :type Float%20%28single-precision%29)))

(fn ConstructionScript
  (bind _bookscale (Variables|Default|GetBookScale))
  (if (Variables|Default|GetAdd%20Books)
    (for (_array_element _array_index) (Variables|Default|GetShelfFromBottom_Zval)
      (switch int (Utilities|Array|Get(acopy) (Variables|Default|GetShelfRowOption) _array_index)
        (:Default)
        (:0)
        (:1
          ;[1 1 1] Row option 1: fill entire shelf with books
          (for (_array_element_2 _array_index_2) (Variables|Default|GetShelfColumnFromRight_Yval)
            (for _index (range 0 (Utilities|Array|Get(acopy) (Variables|Default|GetMaxNumberOfBooksMinusOne) _array_index_2))
              (if (Variables|Default|GetBookOption1)
                (bind _returnvalue (AddComponent|AddStaticMeshComponent false (Math|Transform|MakeTransform (Math|Vector|MakeVector (Variables|Default|GetShelfProtrusion_Xval) (+ (* _index (* (Variables|Default|GetBookBaseWidth) (Variables|Default|GetBookScale))) _array_element_2) _array_element) (Variables|Default|GetBookStandingTall) (Math|Vector|MakeVector _bookscale _bookscale _bookscale))))
                (if (Variables|Default|GetBookOption2)
                  (Rendering|Material|SetMaterial _returnvalue 0 "/Game/VengeanceRising/LibraryLevel/ImportedFromFreeLibrary/Books/Materials/MI_book1_a.MI_book1_a")
                  (else
                    (Rendering|Material|SetMaterial _returnvalue 0 "/Game/VengeanceRising/LibraryLevel/ImportedFromFreeLibrary/Books/Materials/MI_book1_b.MI_book1_b")))
                (else
                  (bind _returnvalue_2 (AddComponent|AddStaticMeshComponent false (Math|Transform|MakeTransform (Math|Vector|MakeVector (Variables|Default|GetShelfProtrusion_Xval) (+ (* _index (* (Variables|Default|GetBookBaseWidth) (Variables|Default|GetBookScale))) _array_element_2) _array_element) (Variables|Default|GetBookStandingTall) (Math|Vector|MakeVector _bookscale _bookscale _bookscale))))
                  (if (Variables|Default|GetBookOption2)
                    (Rendering|Material|SetMaterial _returnvalue_2 5 "/Game/VengeanceRising/LibraryLevel/ImportedFromFreeLibrary/Books/Materials/MI_book1_a.MI_book1_a")
                    (else
                      (Rendering|Material|SetMaterial _returnvalue_2 5 "/Game/VengeanceRising/LibraryLevel/ImportedFromFreeLibrary/Books/Materials/MI_book1_b.MI_book1_b"))))))))))))