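; BP_Sheet is an interactable dining hall level actor that speaks a line of dialogue through a speech bubble.
; Interact requests a box at a spawn offset with an "Interact" label, and ActivateOption calls Talk with the current conversation index.
; Talk casts the child actor to BP_SpeechBubble2 and passes it the matching Conversation entry.
; Thinking is a stub returning false, and the event graph is unused.
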(event EventBeginPlay)

(event EventActorBeginOverlap
  (params (OtherActor :type Actor%20Object%20Reference)))

(event EventTick
  (params (DeltaSeconds :type Float%20%28single-precision%29)))

(fn ConstructionScript)

(fn ActivateOption
  (CallFunction|Talk (Variables|Default|GetConvoIndex))
  (return 0))

(fn Interact
  (return true (Variables|Default|GetSpawn%20Offset) "Interact"))

(fn Talk
  (params (Index :type Integer))
  (bind _asbp_speech_bubble_2 (Utilities|Casting|CastToBP_SpeechBubble2 (Variables|/Script/Engine.ChildActorComponent|GetChildActor (Variables|Default|GetSpeechBubble)))
    (:then
      (Default|Speak _asbp_speech_bubble_2 (Utilities|Array|Get(acopy) (Variables|Default|GetConversation) Index)))
    (:CastFailed
      _))
  (return false))

(fn Thinking
  (return false))