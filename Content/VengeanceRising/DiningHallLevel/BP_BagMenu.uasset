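; BP_BagMenu is an interactable bag in the dining hall level that lets the player open their inventory.
; Interact spawns a BP_Options actor, attaches it to the Bag component at an offset, and registers itself with an "Open" menu entry.
; ActivateOption casts the player pawn to BP_DiningHallPlayer and calls OpenInventory.
; Talk and Thinking are stubs that return false.
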(event Custom|AttachOption
  (bind _returnvalue (Game|SpawnActorfromClass "/Game/VengeanceRising/Brendan/BP_Options.BP_Options_C" (Math|Transform|MakeTransform (+ (Variables|/Script/Engine.SceneComponent|GetRelativeLocation (Variables|Default|GetBag)) "-5.000000,25.000000,60.000000") "0, 0, 0" "1,1,1") "Undefined" 0 0))
  (Class|Actor|AttachRootComponentto _returnvalue (Variables|Default|GetBag) "None" "KeepRelativeOffset" true)
  (Default|AttachItem _returnvalue self "Open" true))

(event EventActorBeginOverlap
  (params (OtherActor :type Actor%20Object%20Reference)))

(event EventTick
  (params (DeltaSeconds :type Float%20%28single-precision%29)))

(fn ConstructionScript)

(fn ActivateOption
  (bind _asbp_dining_hall_player (Utilities|Casting|CastToBP_DiningHallPlayer (Game|Player|GetPlayerPawn 0))
    (:then
      (Default|OpenInventory _asbp_dining_hall_player))
    (:CastFailed
      _))
  (return 0))

(fn Interact
  (CallFunction|AttachOption)
  (return false "0, 0, 0" ""))

(fn Talk
  (params (Index :type Integer))
  (return false))

(fn Thinking
  (return false))