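; BP_Shaker is a pickup item, filed under the dining hall level, that the player can collect into the inventory.
; Interact fetches the item details, adds the item to VengeanceRisingGameInstance, prints a confirmation and destroys the actor.
; GetDetails returns the item with a CanPickUp flag, setting IsPickedUp so only the first query reports true, though Interact does not check that flag.
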(event EventBeginPlay)

(event EventActorBeginOverlap
  (params (OtherActor :type Actor%20Object%20Reference)))

(event EventTick
  (params (DeltaSeconds :type Float%20%28single-precision%29)))

(fn ConstructionScript)

(fn GetDetails
  (bind _item (Variables|Default|GetItem))
  (if (Variables|Default|GetisPickedUp)
    (return _item false)
    (else
      (bind _output_get (Variables|Default|SetisPickedUp true))
      (return _item _output_get))))

(fn Interact
  (bind _self self)
  (bind _item (Class|BPIItemPickUp|GetDetails(Message) _self))
  (bind _asvengeance_rising_game_instance (Utilities|Casting|CastToVengeanceRisingGameInstance (Game|GetGameInstance))
    (:then
      (Default|AddItem _asvengeance_rising_game_instance _item)
      (Development|PrintString (Utilities|String|Append (Utilities|GetDisplayName _self) " was put in the inventory"))
      (Actor|DestroyActor))
    (:CastFailed
      _))
  (return 1))