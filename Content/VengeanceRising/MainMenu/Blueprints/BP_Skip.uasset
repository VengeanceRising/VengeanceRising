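; BP_Skip is an interactable actor that offers a "Skip" option, sending the player on to the Mainhall level.
; Its interaction functions supply the prompt box and label, while the outline, talk and thinking functions simply return false.
; Activating the option fades the first BP_DiningHallPlayer to black, then fires the Go event, which opens the level by name after a short delay.
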(event Custom|Go
  (params (Level :type Name))
  (Utilities|FlowControl|Delay 1.4)
  (Game|OpenLevel(byName) Level))

(event EventBeginPlay)

(event EventActorBeginOverlap
  (params (OtherActor :type Actor%20Object%20Reference)))

(event EventTick
  (params (DeltaSeconds :type Float%20%28single-precision%29)))

(fn ConstructionScript)

(fn ActivateOption
  (bind _outactors (Actor|GetAllActorsOfClass "/Game/VengeanceRising/DiningHallLevel/BP_DiningHallPlayer.BP_DiningHallPlayer_C"))
  (Default|FadetoBlack (Utilities|Array|Get(acopy) _outactors))
  (CallFunction|Go "Mainhall")
  (return 0))

(fn Interact
  (return true (Variables|Default|GetSpawnOffset) "Skip"))

(fn NoOutline
  (return false))

(fn Outline
  (return false))

(fn Talk
  (params (Index :type Integer))
  (return false))

(fn Thinking
  (return false))