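; BP_WoodenCrate is an interactable wooden crate that gives the player a thought as a subtitle.
; Interact casts the player pawn to BP_DiningHallPlayer and passes the Thoughts entry at ThoughtIndex to DisplaySubtitles, without changing the index.
; GetDetails, Talk and Thinking are empty stubs, with the latter two returning false, and the event graph and construction script do nothing.
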(event EventBeginPlay)

(event EventActorBeginOverlap
  (params (OtherActor :type Actor%20Object%20Reference)))

(event EventTick
  (params (DeltaSeconds :type Float%20%28single-precision%29)))

(fn ConstructionScript)

(fn GetDetails
  (return ""))

(fn Interact
  (bind _asbp_dining_hall_player (Utilities|Casting|CastToBP_DiningHallPlayer (Game|Player|GetPlayerPawn 0))
    (:then
      (Default|DisplaySubtitles _asbp_dining_hall_player (Utilities|Array|Get(acopy) (Variables|Default|GetThoughts) (Variables|Default|GetThought%20Index))))
    (:CastFailed
      _))
  (return 0))

(fn Talk
  (params (Index :type Integer))
  (return false))

(fn Thinking
  (return false))