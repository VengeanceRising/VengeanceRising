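; Intro-level story actor that types out narrative paragraphs on a BPW_Story widget shown by its StoryPage widget component.
; Interact starts PlayStory, a delay-driven loop that reveals text letter by letter, appending each finished paragraph and pausing before the next.
; SkipStory sets a flag that halts the loop and shows the first three paragraphs at once.
; Other interaction functions, such as Talk, Outline and Thinking, are stubs.
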(event Custom|PlayStory
  (bind _text (Variables|Default|GetText))
  (bind _paragraphindex (Variables|Default|GetParagraphIndex))
  (bind _paragraphindex_2 (Variables|Default|GetParagraphIndex))
  (bind _item (Utilities|Array|Get(acopy) _text _paragraphindex))
  (if (not (Variables|Default|GetisSkipped)) :!label _label
    (Default|SetText (Variables|Default|GetWidgetRef) (Utilities|Text|ToText(String) (Utilities|String|Append (Variables|Default|GetCurrentText) (Utilities|String|Left _item (Variables|Default|GetLetterIndex)))))
    (bind _result (Math|Integer|IncrementInt (Variables|Default|GetLetterIndex))
      (:%20%20
        (if (<= _result (Utilities|String|Len _item))
          (Utilities|FlowControl|Delay 0.04)
          (goto _label)
          (else
            (Variables|Default|SetLetterIndex 0)
            (Variables|Default|SetCurrentText (Utilities|String|Append (Variables|Default|GetCurrentText) (Utilities|Array|Get(acopy) (Variables|Default|GetText) _paragraphindex_2) " 
 
"))
            (bind _result_2 (Math|Integer|IncrementInt _paragraphindex_2)
              (:%20%20
                (if (<= _result_2 3)
                  (Utilities|FlowControl|Delay 1.5)
                  (goto _label))))))))))

(event Custom|SkipStory
  (bind _text (Variables|Default|GetText))
  (Variables|Default|SetisSkipped true)
  (Default|SetText (Variables|Default|GetWidgetRef) (Utilities|Text|ToText(String) (Utilities|String|Append (Utilities|Array|Get(acopy) _text) " 
 
" (Utilities|Array|Get(acopy) _text 1) " 
 
" (Utilities|Array|Get(acopy) _text 2)))))

(event EventBeginPlay
  (bind _asbpw_story (Utilities|Casting|CastToBPW_Story (UserInterface|GetUserWidgetObject (Variables|Default|GetStoryPage))))
  (Variables|Default|SetWidgetRef _asbpw_story))

(event Collision|EventActorBeginOverlap
  (params (OtherActor :type Actor%20Object%20Reference)))

(event EventTick
  (params (DeltaSeconds :type Float%20%28single-precision%29)))

(fn ConstructionScript)

(fn ActivateOption
  (return 0))

(fn Interact
  (CallFunction|PlayStory)
  (return false "0, 0, 0" ""))

(fn NoOutline
  (return false))

(fn Outline
  (return false))

(fn Talk
  (params (Index :type Integer))
  (return false))

(fn Thinking
  (return false))