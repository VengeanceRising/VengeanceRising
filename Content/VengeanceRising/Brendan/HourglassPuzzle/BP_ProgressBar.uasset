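; Progress bar actor for the hourglass puzzle, showing accumulated time against a target time.
; UpdateTime runs the Rise timeline to lift TimeStand in proportion to the time passed, then updates the running total and rewinds while below target.
; An exact match plays a buzzer, advances the game instance checkpoint and transitions level through the player.
; Overshooting turns the target text red and shows a reset message, without performing the reset here.
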(event Custom|UpdateTime
  (params (TimePassed :type Integer))
  (bind _returnvalue (Math|Conversions|ToFloat(Integer) TimePassed))
  (bind _totallength (Variables|Default|GetTotalLength))
  (bind _targettime (Variables|Default|GetTargetTime))
  (bind _targettime_2 (Variables|Default|GetTargetTime))
  (bind _returnvalue_2 (Math|Conversions|ToFloat(Integer) _targettime))
  (bind _returnvalue_3 (/ _returnvalue _returnvalue_2))
  (bind _returnvalue_4 (* _returnvalue_3 _totallength))
  (bind _data (Timeline|Rise Play)
    (:Update
      (Transformation|SetWorldLocation (Variables|Default|GetTimeStand) (+ (* (Math|Vector|MakeVector 0.0 0.0 _returnvalue_4) _data) (Variables|Default|GetCurrentPos)) false false))
    (:Finished
      (Variables|Default|SetCurrentPos (+ (Variables|Default|GetCurrentPos) (Math|Vector|MakeVector 0.0 0.0 _returnvalue_4)))
      (Variables|Default|SetCurrentTime (+ TimePassed (Variables|Default|GetCurrentTime)))
      (Rendering|Components|TextRender|SetText (Variables|Default|GetTime) (Utilities|Text|ToText(Integer) (Variables|Default|GetCurrentTime)))
      (if (< (Variables|Default|GetCurrentTime) _targettime_2)
        (Timeline|Rise SetNewTime)
        (else
          (bind _asbp_hourglass_player (Utilities|Casting|CastToBP_HourglassPlayer (Game|Player|GetPlayerPawn 0)))
          (if (== (Variables|Default|GetCurrentTime) _targettime_2)
            (Audio|SpawnSoundatLocation "/Game/VengeanceRising/Brendan/Correct_Buzzer.Correct_Buzzer" (Transformation|GetWorldLocation (Variables|Default|GetTargetStand)))
            (Default|Thinking _asbp_hourglass_player "Nicely Done!  All in good time ... get it, TIME.")
            (Utilities|FlowControl|Delay 2.0)
            (bind _asvengeance_rising_game_instance (Utilities|Casting|CastToVengeanceRisingGameInstance (Game|GetGameInstance)))
            (bind _output_get (Variables|Default|SetLevelToGo (Utilities|String|StringToName (Variables|/Game/VengeanceRising/VengeanceRisingGameInstance.VengeanceRisingGameInstance_C|GetCurrentLevel _asvengeance_rising_game_instance))))
            (Default|NextCheckpoint _asvengeance_rising_game_instance)
            (Default|UpdateCurrentLevel _asvengeance_rising_game_instance)
            (Default|LevelTransit _asbp_hourglass_player _output_get)
            (else
              (Rendering|Components|TextRender|SetTextRenderColor (Variables|Default|GetTarget) (Math|Conversions|ToColor(LinearColor) "(R=1.000000,G=0.000000,B=0.000000,A=1.000000)"))
              (Default|Thinking _asbp_hourglass_player "Oh no. We have surpassed the time needed. Let's reset the puzzle."))))))))

(event EventBeginPlay
  (Variables|Default|SetCurrentPos (Transformation|GetWorldLocation (Variables|Default|GetTimeStand))))

(event EventActorBeginOverlap
  (params (OtherActor :type Actor%20Object%20Reference)))

(event EventTick
  (params (DeltaSeconds :type Float%20%28single-precision%29)))

(fn ConstructionScript
  (Rendering|Components|TextRender|SetText (Variables|Default|GetTarget) (Utilities|Text|ToText(Integer) (Variables|Default|GetTargetTime)))
  (Rendering|Components|TextRender|SetText (Variables|Default|GetTime) (Utilities|Text|ToText(Integer) (Variables|Default|GetCurrentTime))))