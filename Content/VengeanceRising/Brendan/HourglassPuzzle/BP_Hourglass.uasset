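; Hourglass puzzle item that tracks time in its top and bottom halves and shows each amount as text.
; ProgressTime moves time from the current top to the bottom, clamped to the total.
; Flip alternately plays and reverses a timeline that rotates the item and both labels 180 degrees.
; When the timeline finishes it swaps the two amounts and toggles IsFlipped, which keeps each label matched to its physical half.
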(event Custom|ProgressTime
  (params (Time :type Integer))
  (bind _timelefttop (Variables|Default|GetTimeLeftTop))
  (bind _timeleftbtm (Variables|Default|GetTimeLeftBtm))
  (bind _totaltime (Variables|Default|GetTotalTime))
  (bind _output_get (Variables|Default|SetCurTop (Math|Integer|Clamp(Integer) (- (Variables|Default|GetCurTop) Time) 0 _totaltime)))
  (bind _output_get_2 (Variables|Default|SetCurBtm (Math|Integer|Clamp(Integer) (+ (Variables|Default|GetCurBtm) Time) 0 _totaltime)))
  (if (Variables|Default|GetisFlipped)
    (Rendering|Components|TextRender|SetText _timelefttop (Utilities|Text|ToText(Integer) _output_get_2))
    (Rendering|Components|TextRender|SetText _timeleftbtm (Utilities|Text|ToText(Integer) _output_get))
    (else
      (Rendering|Components|TextRender|SetText _timelefttop (Utilities|Text|ToText(Integer) _output_get))
      (Rendering|Components|TextRender|SetText _timeleftbtm (Utilities|Text|ToText(Integer) _output_get_2)))))

(event Custom|Flip
  (bind _initrotation (Variables|Default|GetinitRotation))
  (bind _inittextrotation (Variables|Default|GetinitTextRotation))
  (Utilities|FlowControl|MultiGate false true 0
    (:Out%200
      (bind _data (Timeline|FlipHourglass Play)
        (:Update
          (Transformation|SetRelativeRotation (Variables|Default|GetItemScene) (Math|Rotator|MakeRotator (.roll _initrotation) (* _data 1.8e+02) (.yaw _initrotation)) false false)
          (Transformation|SetRelativeRotation (Variables|Default|GetTimeLeftTop) (Math|Rotator|MakeRotator (* _data 1.8e+02) (.pitch _inittextrotation) (.yaw _inittextrotation)) false false)
          (Transformation|SetRelativeRotation (Variables|Default|GetTimeLeftBtm) (Math|Rotator|MakeRotator (* _data 1.8e+02) (.pitch _inittextrotation) (.yaw _inittextrotation)) false false))
        (:Finished
          (Variables|Default|Settemp (Variables|Default|GetCurBtm))
          (Variables|Default|SetCurBtm (Variables|Default|GetCurTop))
          (Variables|Default|SetCurTop (Variables|Default|Gettemp))
          (Variables|Default|SetisFlipped (not (Variables|Default|GetisFlipped))))))
    (:Out%201
      (Timeline|FlipHourglass ReverseFromEnd))))

(event EventBeginPlay
  (bind _totaltime (Variables|Default|GetTotalTime))
  (bind _timeleftbtm (Variables|Default|GetTimeLeftBtm))
  (Variables|Default|SetTimeLeft _totaltime)
  (bind _output_get (Variables|Default|SetCurTop _totaltime))
  (bind _output_get_2 (Variables|Default|SetCurBtm 0))
  (Rendering|Components|TextRender|SetText (Variables|Default|GetTimeLeftTop) (Utilities|Text|ToText(Integer) _output_get))
  (Rendering|Components|TextRender|SetText _timeleftbtm (Utilities|Text|ToText(Integer) _output_get_2))
  (Variables|Default|SetinitRotation (Variables|/Script/Engine.SceneComponent|GetRelativeRotation (Variables|Default|GetItemScene)))
  (Variables|Default|SetinitTextRotation (Variables|/Script/Engine.SceneComponent|GetRelativeRotation _timeleftbtm)))

(fn ConstructionScript)