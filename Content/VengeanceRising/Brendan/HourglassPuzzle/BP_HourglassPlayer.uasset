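; BP_HourglassPlayer is the hourglass puzzle player, selecting objects by gaze dwell from the VR camera.
; Each tick it traces along the view, moves the Reticle to the hit and accumulates hover time while the hit actor stays the same.
; Exceeding HoverDuration sends PressDownMessage to that actor, while a dynamic billboard material shows progress.
; Axis inputs rotate the view; the view-angle limit nodes are unconnected.
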(event EventTick
  (params (DeltaSeconds :type Float%20%28single-precision%29))
  (bind (_location _forward_vector) (CallFunction|GetPlayerVRCameraProperties))
  (bind _outhit (Collision|LineTraceByChannel _location (+ (* _forward_vector 1e+04) _location) "TraceTypeQuery1" false 0 "None"))
  (Transformation|SetWorldLocation (Variables|Default|GetReticle) (.Location (Collision|BreakHitResult _outhit)) false false)
  (Utilities|FlowControl|Sequence
    (:then_0
      (if (== (Variables|Default|GetGazeActor) (.HitActor (Collision|BreakHitResult _outhit)))
        (bind _output_get (Variables|Default|SetHoverProgress (+ DeltaSeconds (Variables|Default|GetHoverProgress))))
        (if (> _output_get (Variables|Default|GetHoverDuration))
          (Variables|Default|SetHoverProgress 0.0)
          (Class|BPIPressButton|PressDown(Message) (Variables|Default|GetGazeActor)))
        (else
          (Variables|Default|SetHoverProgress 0.0))))
    (:then_1
      (Variables|Default|SetGazeActor (.HitActor (Collision|BreakHitResult _outhit)))
      (Rendering|Material|SetScalarParameterValue (Variables|Default|GetReticleDMI) "Progress" (/ (Variables|Default|GetHoverProgress) (Variables|Default|GetHoverDuration)) :!class /Script/Engine.MaterialInstanceDynamic))))

(event EventBeginPlay
  ;[1 1 1] Setting max turn radius
)

(event Input|AxisEvents|InputAxisLookUpRate
  (params (AxisValue :type Float%20%28single-precision%29))
  ;[1 1 1] Rotating View
  (Pawn|Input|AddControllerPitchInput (* AxisValue (Variables|Default|GetBaseLookUpRate) (Utilities|Time|GetWorldDeltaSeconds))))

(event Input|AxisEvents|InputAxisTurnRate
  (params (AxisValue :type Float%20%28single-precision%29))
  ;[1 1 1] Rotating View
  (Pawn|Input|AddControllerYawInput (* AxisValue (Variables|Default|GetBaseTurnRate) (Utilities|Time|GetWorldDeltaSeconds))))

(event Input|AxisEvents|InputAxisTurn
  (params (AxisValue :type Float%20%28single-precision%29))
  ;[1 1 1] Rotating View
  (Pawn|Input|AddControllerYawInput (/ AxisValue 1.0)))

(event Input|AxisEvents|InputAxisLookUp
  (params (AxisValue :type Float%20%28single-precision%29))
  ;[1 1 1] Rotating View
  (Pawn|Input|AddControllerPitchInput (/ AxisValue 1.0)))

(fn ConstructionScript
  (bind _dynamic_material (CallFunction|CreateDynamicBillboardMaterial (Variables|Default|GetReticle)))
  (Variables|Default|SetReticleDMI _dynamic_material))