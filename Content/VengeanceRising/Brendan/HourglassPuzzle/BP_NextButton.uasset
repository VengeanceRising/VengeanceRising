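; BP_NextButton is the button in the hourglass puzzle that skips time forward to when the next running hourglass empties.
; Pressing it plays a click, then GetProgress finds the smallest non-zero top amount across AllHourglasses, using 100 as a "none running" sentinel.
; If one is found, it updates the ProgressBar by that amount, plays a sand-pouring sound and advances every hourglass equally.
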(event Custom|GetProgress
  (bind _allhourglasses (Variables|Default|GetAllHourglasses))
  (for _array_element _allhourglasses
    (if (!= (Variables|/Game/VengeanceRising/Brendan/HourglassPuzzle/BP_Hourglass.BP_Hourglass_C|GetCurTop _array_element) 0)
      (Variables|Default|SetSmallestTimeLeft (Math|Integer|Min(Integer) (Variables|Default|GetSmallestTimeLeft) (Variables|/Game/VengeanceRising/Brendan/HourglassPuzzle/BP_Hourglass.BP_Hourglass_C|GetCurTop _array_element)))))
  (if (== (Variables|Default|GetSmallestTimeLeft) 100)
    (Variables|Default|SetSmallestTimeLeft 100)
    (else
      (Default|UpdateTime (Variables|Default|GetProgressBar) (Variables|Default|GetSmallestTimeLeft))
      (Audio|SpawnSoundatLocation "/Game/VengeanceRising/Brendan/Sounds/sand-pouring-2sec.sand-pouring-2sec" "0, 0, 0")
      (for _array_element_2 _allhourglasses
        (Default|ProgressTime _array_element_2 (Variables|Default|GetSmallestTimeLeft)))
      (Variables|Default|SetSmallestTimeLeft 100))))

(event EventBeginPlay)

(event Collision|EventActorBeginOverlap
  (params (OtherActor :type Actor%20Object%20Reference)))

(event EventTick
  (params (DeltaSeconds :type Float%20%28single-precision%29)))

(fn ConstructionScript)

(fn PressDown
  (Audio|SpawnSoundAttached "/Game/VengeanceRising/Brendan/Button_Sound.Button_Sound" (Variables|Default|GetButton))
  (CallFunction|GetProgress)
  (return false))