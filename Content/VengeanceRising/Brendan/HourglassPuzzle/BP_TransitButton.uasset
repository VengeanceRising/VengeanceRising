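; A button actor that travels to another level when its Press Down function is called.
; The construction script applies the configurable label text and stretches the button's X scale by a size multiplier.
; Press Down opens the level named in Level, except that the value "Back" opens the CurrentLevel stored in VengeanceRisingGameInstance.
; The event graph is unused, so the press must be triggered from outside.
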(event EventBeginPlay)

(event Collision|EventActorBeginOverlap
  (params (OtherActor :type Actor%20Object%20Reference)))

(event EventTick
  (params (DeltaSeconds :type Float%20%28single-precision%29)))

(fn ConstructionScript
  (bind _button (Variables|Default|GetButton))
  (bind _returnvalue (Transformation|GetWorldScale _button))
  (Rendering|Components|TextRender|SetText (Variables|Default|GetText) (Variables|Default|GetButtonText))
  (Transformation|SetWorldScale3D _button (Math|Vector|MakeVector (* (Variables|Default|GetSizeMultiplier) (.x _returnvalue)) (.y _returnvalue) (.z _returnvalue))))

(fn PressDown
  (if (Utilities|Name|Equal(Name) (Variables|Default|GetLevel) "Back")
    (bind _asvengeance_rising_game_instance (Utilities|Casting|CastToVengeanceRisingGameInstance (Game|GetGameInstance))
      (:then
        (Game|OpenLevel(byName) (Utilities|String|StringToName (Variables|/Game/VengeanceRising/VengeanceRisingGameInstance.VengeanceRisingGameInstance_C|GetCurrentLevel _asvengeance_rising_game_instance))))
      (:CastFailed
        _))
    (else
      (Game|OpenLevel(byName) (Variables|Default|GetLevel))))
  (return false))