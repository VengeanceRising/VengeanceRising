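; 3D inventory details panel that previews selected items, fills twelve BP_Item child-actor slots and offers a combine mode.
; ShowDetails and ShowItem2 set the preview meshes, with ShowDetails also feeding name and description to the widget.
; CombineMode toggles widget and component visibility, playing or reversing the Rearrange timeline to move item and buttons from stored origins.
; Tick converts slider height into a scale value passed to BP_InventoryPlayer.
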(event Custom|ShowItem2
  (params (Item :type BPS%20Item%20Structure))
  (bind (_name _description _thumbnail _mesh _sizemultiplier) (Utilities|Struct|BreakBPS_Item Item))
  (bind _item2 (Variables|Default|GetItem2))
  (Components|StaticMesh|SetStaticMesh _item2 _mesh)
  (Transformation|SetWorldScale3D _item2 (* "1.000000,1.000000,1.000000" _sizemultiplier)))

(event Custom|ShowDetails
  (params (Item :type BPS%20Item%20Structure))
  (bind (_name _description _thumbnail _mesh _sizemultiplier) (Utilities|Struct|BreakBPS_Item Item))
  (bind _itemd (Variables|Default|GetItemD))
  (Variables|/Game/VengeanceRising/Brendan/InventoryInterface/BPW_ItemDetails.BPW_ItemDetails_C|SetName _itemd _name)
  (Variables|/Game/VengeanceRising/Brendan/InventoryInterface/BPW_ItemDetails.BPW_ItemDetails_C|SetDescription _itemd _description)
  (Components|StaticMesh|SetStaticMesh (Variables|Default|GetItem) _mesh)
  (Transformation|SetWorldScale3D (Variables|Default|GetItem) (* "1.000000,1.000000,1.000000" _sizemultiplier)))

(event Custom|updateOrigin
  (Variables|Default|SetCombineOrigin (Transformation|GetWorldLocation (Variables|Default|GetCombineButton)))
  (Variables|Default|SetItem1Origin (Transformation|GetWorldLocation (Variables|Default|GetItem)))
  (Variables|Default|SetCancelOrigin (Transformation|GetWorldLocation (Variables|Default|GetCancelButton))))

(event Custom|SpawnItem
  (params (Item :type BPS%20Item%20Structure))
  (Default|SetItem (Utilities|Array|Get(acopy) (Variables|Default|GetSlotArray) (Variables|Default|GetemptySlot)) Item)
  (Variables|Default|SetemptySlot (+ (Variables|Default|GetemptySlot) 1)))

(event Custom|CombineMode
  (bind _item2 (Variables|Default|GetItem2))
  (bind _item (Variables|Default|GetItem))
  (Rendering|ToggleVisibility (Variables|Default|GetScale) true)
  (Rendering|ToggleVisibility (Variables|Default|GetSlider) false)
  (Default|ToggleWidget (Variables|Default|GetItemD))
  (Rendering|ToggleVisibility (Variables|Default|GetItem2) false)
  (Class|PrimitiveComponent|SetConstraintMode (Variables|Default|GetItem) "CustomPlane")
  (if (Variables|Default|GetisActive)
    (bind (_direction _data1 _data2 _data3) (Timeline|Rearrange ReverseFromEnd)
      (:Update
        (Transformation|SetWorldLocation (Variables|Default|GetCombineButton) (+ (* "-8.000000,-210.000000,-119.000000" _data2) (Variables|Default|GetCombineOrigin)) false false)
        (Transformation|SetWorldLocation _item (+ (* "0.000000,0.000000,150.000000" _data1) (Variables|Default|GetItem1Origin)) false false)
        (Transformation|SetWorldLocation (Variables|Default|GetCancelButton) (+ (* "-100.000000,0.000000,0.000000" _data3) (Variables|Default|GetCancelOrigin)) false false))
      (:Finished
        (Class|PrimitiveComponent|SetConstraintMode _item "Default")
        (Components|StaticMesh|SetStaticMesh _item2 "/Game/Geometry/Meshes/1M_Cube.1M_Cube")
        (Transformation|SetWorldScale3D _item2 "1.000000,1.000000,1.000000")
        (Variables|Default|SetisActive (not (Variables|Default|GetisActive)))))
    (else
      (Timeline|Rearrange Play))))

(event EventBeginPlay
  (bind _asbpw_item_details (Utilities|Casting|CastToBPW_ItemDetails (UserInterface|GetUserWidgetObject (Variables|Default|GetItemDetails))))
  (Variables|Default|SetItemD _asbpw_item_details)
  (Variables|Default|SetZeroing (.z (Transformation|GetWorldLocation (Variables|Default|GetSlider))))
  (CallFunction|UpdateOrigin))

(event EventTick
  (params (DeltaSeconds :type Float%20%28single-precision%29))
  (bind _output_get (Variables|Default|SetScaleVal (* (/ (- (.z (Transformation|GetWorldLocation (Variables|Default|GetSlider))) (Variables|Default|GetZeroing)) 142.0) 1e+02)))
  (bind _asbp_inventory_player (Utilities|Casting|CastToBP_InventoryPlayer (Game|Player|GetPlayerPawn 0)))
  (Default|ScaleItem _asbp_inventory_player _output_get))

(fn ConstructionScript
  (bind _asbp_item (Utilities|Casting|CastToBP_Item (Variables|/Script/Engine.ChildActorComponent|GetChildActor (Variables|Default|GetSlot1))))
  (bind _asbp_item_2 (Utilities|Casting|CastToBP_Item (Variables|/Script/Engine.ChildActorComponent|GetChildActor (Variables|Default|GetSlot2))))
  (bind _asbp_item_3 (Utilities|Casting|CastToBP_Item (Variables|/Script/Engine.ChildActorComponent|GetChildActor (Variables|Default|GetSlot3))))
  (bind _asbp_item_4 (Utilities|Casting|CastToBP_Item (Variables|/Script/Engine.ChildActorComponent|GetChildActor (Variables|Default|GetSlot4))))
  (bind _asbp_item_5 (Utilities|Casting|CastToBP_Item (Variables|/Script/Engine.ChildActorComponent|GetChildActor (Variables|Default|GetSlot5))))
  (bind _asbp_item_6 (Utilities|Casting|CastToBP_Item (Variables|/Script/Engine.ChildActorComponent|GetChildActor (Variables|Default|GetSlot6))))
  (bind _asbp_item_7 (Utilities|Casting|CastToBP_Item (Variables|/Script/Engine.ChildActorComponent|GetChildActor (Variables|Default|GetSlot7))))
  (bind _asbp_item_8 (Utilities|Casting|CastToBP_Item (Variables|/Script/Engine.ChildActorComponent|GetChildActor (Variables|Default|GetSlot8))))
  (bind _asbp_item_9 (Utilities|Casting|CastToBP_Item (Variables|/Script/Engine.ChildActorComponent|GetChildActor (Variables|Default|GetSlot9))))
  (bind _asbp_item_10 (Utilities|Casting|CastToBP_Item (Variables|/Script/Engine.ChildActorComponent|GetChildActor (Variables|Default|GetSlot10))))
  (bind _asbp_item_11 (Utilities|Casting|CastToBP_Item (Variables|/Script/Engine.ChildActorComponent|GetChildActor (Variables|Default|GetSlot11))))
  (bind _asbp_item_12 (Utilities|Casting|CastToBP_Item (Variables|/Script/Engine.ChildActorComponent|GetChildActor (Variables|Default|GetSlot12))))
  (Variables|Default|SetSlotArray (Utilities|Array|MakeArray _asbp_item _asbp_item_2 _asbp_item_3 _asbp_item_4 _asbp_item_5 _asbp_item_6 _asbp_item_7 _asbp_item_8 _asbp_item_9 _asbp_item_10 _asbp_item_11 _asbp_item_12)))