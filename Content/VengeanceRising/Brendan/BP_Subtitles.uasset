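; BP_Subtitles is an actor that shows and hides subtitle text, such as a thought, through a SubBox widget component.
; On BeginPlay it casts the component's user widget to BPW_Subtitles and caches it.
; The Thinking event passes the given text to the widget and makes SubBox visible, while CloseSubBox clears the text and hides it.
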(event Custom|Thinking
  (params (Thought :type Text))
  (Default|DisplayText (Variables|Default|GetSubtitleWidget) Thought)
  (Rendering|SetVisibility (Variables|Default|GetSubBox) true false))

(event Custom|CloseSubBox
  (Default|DisplayText (Variables|Default|GetSubtitleWidget))
  (Rendering|SetVisibility (Variables|Default|GetSubBox) false false))

(event EventBeginPlay
  (bind _asbpw_subtitles (Utilities|Casting|CastToBPW_Subtitles (UserInterface|GetUserWidgetObject (Variables|Default|GetSubBox))))
  (Variables|Default|SetSubtitleWidget _asbpw_subtitles))

(event EventActorBeginOverlap
  (params (OtherActor :type Actor%20Object%20Reference)))

(event EventTick
  (params (DeltaSeconds :type Float%20%28single-precision%29)))

(fn ConstructionScript)