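; BP_SpeechBubble is an actor that shows timed speech text in a Bubble widget component.
; On BeginPlay it caches the component's BPW_Speech widget, which renders the text.
; Speak displays the given text and reveals the bubble, then clears and hides it after a fixed ten-second delay.
; CloseBubble clears and hides it immediately.
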(event Custom|CloseBubble
  (Default|DisplayText (Variables|Default|GetSpeechWidget))
  (Rendering|SetVisibility (Variables|Default|GetBubble) false false))

(event Custom|Speak
  (params (Speech :type Text))
  (bind _bubble (Variables|Default|GetBubble))
  (bind _speechwidget (Variables|Default|GetSpeechWidget))
  (Default|DisplayText _speechwidget Speech)
  (Rendering|SetVisibility _bubble true false)
  (Utilities|FlowControl|Delay 1e+01)
  (Default|DisplayText _speechwidget)
  (Rendering|SetVisibility _bubble false false))

(event EventBeginPlay
  (bind _asbpw_speech (Utilities|Casting|CastToBPW_Speech (UserInterface|GetUserWidgetObject (Variables|Default|GetBubble))))
  (Variables|Default|SetSpeechWidget _asbpw_speech))

(event EventActorBeginOverlap
  (params (OtherActor :type Actor%20Object%20Reference)))

(event EventTick
  (params (DeltaSeconds :type Float%20%28single-precision%29)))

(fn ConstructionScript)