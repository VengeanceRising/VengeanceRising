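; BP_AnswerSheet is a clue-interface answer pane holding ten BP_CheckBox child actors for recording an answer.
; The construction script casts the child actors into a CheckBoxes array, which BeginPlay numbers 1 to 10 after hiding the pane.
; ShowPane and HidePane toggle visibility and collision on the sheet and every checkbox together.
; GetAnswer returns the numbers of checkboxes whose ToggleIndex is 1.
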(event Custom|ShowPane
  (Rendering|SetActorHiddenInGame false)
  (Collision|SetActorEnableCollision true)
  (for _array_element (Variables|Default|GetCheckBoxes)
    (Rendering|SetActorHiddenInGame _array_element false)
    (Collision|SetActorEnableCollision _array_element true)))

(event Custom|HidePane
  (Rendering|SetActorHiddenInGame true)
  (Collision|SetActorEnableCollision false)
  (for _array_element (Variables|Default|GetCheckBoxes)
    (Rendering|SetActorHiddenInGame _array_element true)
    (Collision|SetActorEnableCollision _array_element false)))

(event EventActorBeginOverlap
  (params (OtherActor :type Actor%20Object%20Reference)))

(event EventTick
  (params (DeltaSeconds :type Float%20%28single-precision%29)))

(event EventBeginPlay
  (CallFunction|HidePane)
  (for (_array_element _array_index) (Variables|Default|GetCheckBoxes)
    (Variables|/Game/VengeanceRising/Brendan/ClueInterface/BP_CheckBox.BP_CheckBox_C|SetCheckBoxNumber _array_element (+ _array_index 1)) ; Number the checkboxes 1 to 10
  ))

(fn ConstructionScript
  (bind _asbp_check_box (Utilities|Casting|CastToBP_CheckBox (Variables|/Script/Engine.ChildActorComponent|GetChildActor (Variables|Default|GetCheck1))))
  (bind _asbp_check_box_2 (Utilities|Casting|CastToBP_CheckBox (Variables|/Script/Engine.ChildActorComponent|GetChildActor (Variables|Default|GetCheck2))))
  (bind _asbp_check_box_3 (Utilities|Casting|CastToBP_CheckBox (Variables|/Script/Engine.ChildActorComponent|GetChildActor (Variables|Default|GetCheck3))))
  (bind _asbp_check_box_4 (Utilities|Casting|CastToBP_CheckBox (Variables|/Script/Engine.ChildActorComponent|GetChildActor (Variables|Default|GetCheck4))))
  (bind _asbp_check_box_5 (Utilities|Casting|CastToBP_CheckBox (Variables|/Script/Engine.ChildActorComponent|GetChildActor (Variables|Default|GetCheck5))))
  (bind _asbp_check_box_6 (Utilities|Casting|CastToBP_CheckBox (Variables|/Script/Engine.ChildActorComponent|GetChildActor (Variables|Default|GetCheck6))))
  (bind _asbp_check_box_7 (Utilities|Casting|CastToBP_CheckBox (Variables|/Script/Engine.ChildActorComponent|GetChildActor (Variables|Default|GetCheck7))))
  (bind _asbp_check_box_8 (Utilities|Casting|CastToBP_CheckBox (Variables|/Script/Engine.ChildActorComponent|GetChildActor (Variables|Default|GetCheck8))))
  (bind _asbp_check_box_9 (Utilities|Casting|CastToBP_CheckBox (Variables|/Script/Engine.ChildActorComponent|GetChildActor (Variables|Default|GetCheck9))))
  (bind _asbp_check_box_10 (Utilities|Casting|CastToBP_CheckBox (Variables|/Script/Engine.ChildActorComponent|GetChildActor (Variables|Default|GetCheck10))))
  (Variables|Default|SetCheckBoxes (Utilities|Array|MakeArray _asbp_check_box _asbp_check_box_2 _asbp_check_box_3 _asbp_check_box_4 _asbp_check_box_5 _asbp_check_box_6 _asbp_check_box_7 _asbp_check_box_8 _asbp_check_box_9 _asbp_check_box_10)))

(fn GetAnswer
  (Utilities|Array|Clear (Variables|Default|GetTicks))
  (for _array_element (Variables|Default|GetCheckBoxes)
    (if (== (Variables|/Game/VengeanceRising/Brendan/ClueInterface/BP_CheckBox.BP_CheckBox_C|GetToggleIndex _array_element) 1)
      (Utilities|Array|Add (Variables|Default|GetTicks) (Variables|/Game/VengeanceRising/Brendan/ClueInterface/BP_CheckBox.BP_CheckBox_C|GetCheckBoxNumber _array_element))))
  (return (Variables|Default|GetTicks)))