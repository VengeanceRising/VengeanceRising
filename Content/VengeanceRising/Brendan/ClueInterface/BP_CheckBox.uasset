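; BP_CheckBox is a three-state checkbox actor in the clue interface, cycling between empty, tick and cross.
; Construction creates a dynamic instance of M_CheckBox on the Box component.
; ToggleCheckBox increments ToggleIndex, wrapping back to empty after cross, swaps the CheckStatus texture parameter to match and returns the new index.
; The event graph holds only disabled stubs, so toggling relies on external callers.
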(event EventActorBeginOverlap
  (params (OtherActor :type Actor%20Object%20Reference)))

(event EventTick
  (params (DeltaSeconds :type Float%20%28single-precision%29)))

(fn ConstructionScript
  (bind _returnvalue (Rendering|Material|CreateDynamicMaterialInstance (Variables|Default|GetBox) 0 "/Game/VengeanceRising/Brendan/M_CheckBox.M_CheckBox" :!class /Script/Engine.PrimitiveComponent))
  (Variables|Default|SetTextureDMI _returnvalue))

(fn ToggleCheckBox
  (bind _texturedmi (Variables|Default|GetTextureDMI))
  (bind _result (Math|Integer|IncrementInt (Variables|Default|GetToggleIndex) :!label _label)
    (:%20%20
      (if (<= _result 2)
        (switch int (Variables|Default|GetToggleIndex)
          (:Default
            (Rendering|Material|SetTextureParameterValue _texturedmi "CheckStatus" "/Game/VengeanceRising/Brendan/empty-blue-checkbox.empty-blue-checkbox" :!label _label_2))
          (:0
            (goto _label_2))
          (:1
            (Rendering|Material|SetTextureParameterValue _texturedmi "CheckStatus" "/Game/VengeanceRising/Brendan/tick-blue-checkbox.tick-blue-checkbox"))
          (:2
            (Rendering|Material|SetTextureParameterValue _texturedmi "CheckStatus" "/Game/VengeanceRising/Brendan/cross-blue-checkbox.cross-blue-checkbox")))
        (return (Variables|Default|GetToggleIndex))
        (else
          (Variables|Default|SetToggleIndex -1)
          (goto _label))))))