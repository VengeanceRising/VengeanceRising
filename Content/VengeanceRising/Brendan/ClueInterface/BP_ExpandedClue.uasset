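; BP_ExpandedClue is an expanded-clue pane actor with a widget component and a color button that cycles through six preset colors.
; BeginPlay caches the BPW_ExpandedClue widget, then hides the pane and disables its collision.
; ShowPane reveals it with a given color index by priming the counter and calling SwitchColor.
; SwitchColor advances and wraps that index, writing the color to the button's dynamic material created in the construction script.
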(event Custom|SwitchColor
  (bind _result (Math|Integer|IncrementInt (Variables|Default|GetToggleColor) :!label _label)
    (:%20%20
      (if (>= _result 6)
        (Variables|Default|SetToggleColor -1)
        (goto _label)
        (else
          (Rendering|Material|SetVectorParameterValue (Variables|Default|GetDMIColor) "Color" (Utilities|Array|Get(acopy) (Utilities|Array|MakeArray (Utilities|Struct|MakeLinearColor 0.15 0.15 0.15 1.0) "(R=0.090842,G=0.300544,B=0.904661,A=1.000000)" "(R=0.879622,G=0.814847,B=0.184475,A=1.000000)" "(R=0.323143,G=0.854993,B=0.238398,A=1.000000)" "(R=0.871367,G=0.473531,B=0.187821,A=1.000000)" "(R=1.000000,G=0.208637,B=0.955973,A=1.000000)") (Variables|Default|GetToggleColor)) :!class /Script/Engine.MaterialInstanceDynamic))))))

(event Custom|HidePane
  (Rendering|SetActorHiddenInGame true)
  (Collision|SetActorEnableCollision false))

(event Custom|ShowPane
  (params (ColorIndex :type Integer))
  (Variables|Default|SetToggleColor (- ColorIndex 1))
  (CallFunction|SwitchColor)
  (Rendering|SetActorHiddenInGame false)
  (Collision|SetActorEnableCollision true))

(event EventBeginPlay
  (bind _asbpw_expanded_clue (Utilities|Casting|CastToBPW_ExpandedClue (UserInterface|GetUserWidgetObject (Variables|Default|GetExpansion))))
  (Variables|Default|SetExClue _asbpw_expanded_clue)
  (CallFunction|HidePane))

(event EventActorBeginOverlap
  (params (OtherActor :type Actor%20Object%20Reference)))

(event EventTick
  (params (DeltaSeconds :type Float%20%28single-precision%29)))

(fn ConstructionScript
  (bind _returnvalue (Rendering|Material|CreateDynamicMaterialInstance (Variables|Default|GetColorButton) 0 "/Game/VengeanceRising/Brendan/M_Color.M_Color" :!class /Script/Engine.PrimitiveComponent))
  (Variables|Default|SetDMIColor _returnvalue))