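; BP_Cluebox is a clue box actor in the clue interface, showing a thumbnail and a classification color, that can be combined with another box.
; Construction creates dynamic materials for color cube and display; InputDetails fills in clue data and updates the thumbnail.
; SwitchColor cycles through six colors.
; A hard enough hit against another box, measured as speed times mass, spawns an explosion, then calls CombineClues on BP_CluePlayerLeap after a short delay.
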(event OnComponentHit(ColorCube)
  (params (OtherActor :type Actor%20Object%20Reference) (OtherComp :type Primitive%20Component%20Object%20Reference) (NormalImpulse :type Vector :default "0, 0, 0") (Hit :type Hit%20Result%20Structure%20%28by%20ref%29))
  (bind (_bblockinghit _binitialoverlap _time _location _impactpoint _normal _impactnormal _physmat _hitactor _hitcomponent) (Collision|BreakHitResult Hit))
  (bind (_x _y _z) (Math|Vector|BreakVector _location))
  ;[1 1 1] Activate CombineClues if the collision force is >5000
  (bind _asbp_cluebox (Utilities|Casting|CastToBP_Cluebox _hitactor))
  (if (>= (* (Math|Vector|VectorLength (Transformation|GetComponentVelocity _hitcomponent)) (Physics|GetMass _hitcomponent)) 5e+03)
    (Effects|SpawnEmitteratLocation "/Game/MobileStarterContent/Particles/P_Explosion.P_Explosion" _location)
    (bind _asbp_clue_player_leap (Utilities|Casting|CastToBP_CluePlayerLeap (Game|Player|GetPlayerPawn 0)))
    (Utilities|FlowControl|Delay 0.2)
    (Default|CombineClues _asbp_clue_player_leap self _asbp_cluebox (Math|Vector|MakeVector 641.0 _y _z))))

(event Custom|SwitchColor
  ;[1 1 1] Toggle classification color
  (bind _result (Math|Integer|IncrementInt (Variables|Default|GetToggleColor) :!label _label)
    (:%20%20
      (if (>= _result 6)
        (Variables|Default|SetToggleColor -1)
        (goto _label)
        (else
          (Rendering|Material|SetVectorParameterValue (Variables|Default|GetDMIColor) "Color" (Utilities|Array|Get(acopy) (Utilities|Array|MakeArray (Utilities|Struct|MakeLinearColor 0.15 0.15 0.15 1.0) "(R=0.090842,G=0.300544,B=0.904661,A=1.000000)" "(R=0.879622,G=0.814847,B=0.184475,A=1.000000)" "(R=0.323143,G=0.854993,B=0.238398,A=1.000000)" "(R=0.871367,G=0.473531,B=0.187821,A=1.000000)" "(R=1.000000,G=0.208637,B=0.955973,A=1.000000)") (Variables|Default|GetToggleColor)) :!class /Script/Engine.MaterialInstanceDynamic))))))

(event Custom|InputDetails
  (params (Name :type Text) (Description :type Text) (Thumbnail :type Texture%202D%20Object%20Reference) (ColorIndex :type Integer))
  (Variables|Default|SetName Name)
  (Variables|Default|SetLong%20Description Description)
  (Variables|Default|SetThumbnail Thumbnail)
  (Variables|Default|SetToggleColor ColorIndex)
  (Rendering|Material|SetTextureParameterValue (Variables|Default|GetDMITexture) "ThumbnailPic" (Variables|Default|GetThumbnail)))

(event EventBeginPlay)

(event EventActorBeginOverlap
  (params (OtherActor :type Actor%20Object%20Reference)))

(event EventTick
  (params (DeltaSeconds :type Float%20%28single-precision%29)))

(fn ConstructionScript
  (bind _returnvalue (Rendering|Material|CreateDynamicMaterialInstance (Variables|Default|GetColorCube) 0 "/Game/VengeanceRising/Brendan/M_Color.M_Color" :!class /Script/Engine.PrimitiveComponent))
  (Variables|Default|SetDMIColor _returnvalue)
  (bind _returnvalue_2 (Rendering|Material|CreateDynamicMaterialInstance (Variables|Default|GetDisplay) 0 "/Game/VengeanceRising/Brendan/M_Thumbnail.M_Thumbnail" :!class /Script/Engine.PrimitiveComponent))
  (bind _output_get (Variables|Default|SetDMITexture _returnvalue_2))
  (Rendering|Material|SetTextureParameterValue _output_get "ThumbnailPic" (Variables|Default|GetThumbnail)))