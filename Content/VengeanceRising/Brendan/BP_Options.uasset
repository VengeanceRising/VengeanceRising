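; BP_Options is a short-lived selectable option with a text label, bound to a parent item for VR interaction.
; AttachItem stores the parent, sets the label and sets IsMenu; outside menu mode, Tick turns the cube in yaw and roll toward the VR camera.
; Interact sends ActivateOption to the parent and destroys the actor, which otherwise destroys itself after a five-second delay from BeginPlay.
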(event Custom|AttachItem
  (params (Item :type Actor%20Object%20Reference) (Text :type Text) (isMenu :type Boolean))
  (Variables|Default|SetParentItem Item)
  (Rendering|Components|TextRender|SetText (Variables|Default|GetText) Text)
  (Variables|Default|SetisMenu isMenu))

(event EventBeginPlay)

(event EventActorBeginOverlap
  (params (OtherActor :type Actor%20Object%20Reference)))

(event EventTick
  (params (DeltaSeconds :type Float%20%28single-precision%29)))

(event EventBeginPlay
  (Utilities|FlowControl|Delay 5.0)
  (Actor|DestroyActor))

(event EventTick
  (params (DeltaSeconds :type Float%20%28single-precision%29))
  (bind _cube (Variables|Default|GetCube))
  (if (not (Variables|Default|GetisMenu))
    (bind _location (CallFunction|GetPlayerVRCameraProperties))
    (Transformation|SetWorldRotation _cube (Math|Rotator|MakeRotator (.roll (Math|Rotator|FindLookatRotation (Transformation|GetWorldLocation _cube) _location)) 0.0 (+ (.yaw (Math|Rotator|FindLookatRotation (Transformation|GetWorldLocation _cube) _location)) -9e+01)) false false)))

(fn ConstructionScript)

(fn ActivateOption
  (return 0))

(fn Interact
  (Class|BPIInteract|ActivateOption(Message) (Variables|Default|GetParentItem))
  (Actor|DestroyActor)
  (return false "0, 0, 0" ""))

(fn Talk
  (params (Index :type Integer))
  (return false))

(fn Thinking
  (return false))