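; BP_PopUp2 is a toggleable tutorial pop-up bubble for VR that shows text on a 3D widget component.
; On BeginPlay it caches the bubble's BPW_TutorialOpp widget, and every tick it rotates the bubble to face the player's VR camera.
; TogglePopUp flips visibility with an active flag, pushing its Text to the widget each time the bubble is shown.
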(event Custom|TogglePopUp
  (bind _popupbubble (Variables|Default|GetPopUpBubble))
  (if (Variables|Default|GetisActive)
    (Rendering|SetVisibility _popupbubble false false)
    (Variables|Default|SetisActive false)
    (else
      (Default|DisplayText (Variables|Default|Get3DWidget) (Variables|Default|GetText))
      (Rendering|SetVisibility _popupbubble true false)
      (Variables|Default|SetisActive true))))

(event EventBeginPlay
  (bind _asbpw_tutorial_opp (Utilities|Casting|CastToBPW_TutorialOpp (UserInterface|GetUserWidgetObject (Variables|Default|GetPopUpBubble))))
  (Variables|Default|Set3DWidget _asbpw_tutorial_opp))

(event EventTick
  (params (DeltaSeconds :type Float%20%28single-precision%29))
  (bind _location (CallFunction|GetPlayerVRCameraProperties))
  (Transformation|SetWorldRotation (Variables|Default|GetPopUpBubble) (Math|Rotator|FindLookatRotation (Transformation|GetWorldLocation (Variables|Default|GetPopUpBubble)) _location) false false))

(fn ConstructionScript)