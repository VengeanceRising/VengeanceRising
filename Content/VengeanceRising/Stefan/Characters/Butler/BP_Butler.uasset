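; Butler NPC that bows and speaks a line in a speech bubble when interacted with.
; The construction script fills a one-line Conversation array, and Interact plays the bow animation on the mesh before calling Talk.
; Talk and Converse send lines to a BP_SpeechBubble child actor.
; GetDetails and Thinking are empty stubs, and the event graph is unused.
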(event EventBeginPlay)

(event EventActorBeginOverlap
  (params (OtherActor :type Actor%20Object%20Reference)))

(event EventTick
  (params (DeltaSeconds :type Float%20%28single-precision%29)))

(fn ConstructionScript
  (Variables|Default|SetConversation (Utilities|Array|MakeArray "Yo homie, 'sup?!")))

(fn Converse
  (bind _asbp_speech_bubble (Utilities|Casting|CastToBP_SpeechBubble (Variables|/Script/Engine.ChildActorComponent|GetChildActor (Variables|Default|GetSpeechBubble)))
    (:then
      (Default|Speak _asbp_speech_bubble (Utilities|Array|Get(acopy) (Variables|Default|GetConversation))))
    (:CastFailed
      _))
  (return))

(fn GetDetails
  (return ""))

(fn Interact
  (Components|Animation|PlayAnimation (Variables|Character|GetMesh) "/Game/VengeanceRising/Stefan/Characters/Butler/quick_formal_bow.quick_formal_bow" false)
  (CallFunction|Talk)
  (return 2))

(fn Talk
  (params (Index :type Integer))
  (bind _asbp_speech_bubble (Utilities|Casting|CastToBP_SpeechBubble (Variables|/Script/Engine.ChildActorComponent|GetChildActor (Variables|Default|GetSpeechBubble)))
    (:then
      (Default|Speak _asbp_speech_bubble (Utilities|Array|Get(acopy) (Variables|Default|GetConversation) Index)))
    (:CastFailed
      _))
  (return false))

(fn Thinking
  (return false))