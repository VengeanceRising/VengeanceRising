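; BP_Host is a host character that talks through a child-actor speech bubble and plays a death when interacted with.
; Each tick the bubble yaws toward the player's VR camera, using an offset from the mesh's initial yaw and clamped to a limited arc.
; The first Interact plays a zombie death animation, speaks the first Conversation line via Talk and sets IsDead.
; ActivateOption and Thinking are stubs.
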(event EventBeginPlay
  (Variables|Default|SetRotationOffset (- -9e+01 (.yaw (Transformation|GetWorldRotation (Variables|Character|GetMesh))))))

(event EventTick
  (params (DeltaSeconds :type Float%20%28single-precision%29))
  (bind _location (CallFunction|GetPlayerVRCameraProperties))
  (Transformation|SetRelativeRotation (Variables|Default|GetSpeechBubble) (Math|Rotator|MakeRotator 0.0 0.0 (Math|Float|ClampAngle (+ (.yaw (Math|Rotator|FindLookatRotation (Transformation|GetWorldLocation (Variables|Default|GetSpeechBubble)) _location)) (Variables|Default|GetRotationOffset)) -3e+01 3e+01)) false false))

(fn ConstructionScript)

(fn ActivateOption
  (return 0))

(fn Interact
  (if (Variables|Default|GetIsDead)
    _
    (else
      (Components|Animation|PlayAnimation (Variables|Character|GetMesh) "/Game/VengeanceRising/Commons/Characters/Host/zombie_death.zombie_death" false)
      (CallFunction|Talk)
      (Variables|Default|SetIsDead true)))
  (return false "0, 0, 0" ""))

(fn Talk
  (params (Index :type Integer))
  (bind _asbp_speech_bubble (Utilities|Casting|CastToBP_SpeechBubble (Variables|/Script/Engine.ChildActorComponent|GetChildActor (Variables|Default|GetSpeechBubble)))
    (:then
      (Default|Speak _asbp_speech_bubble (Utilities|Array|Get(acopy) (Variables|Default|GetConversation) Index)))
    (:CastFailed
      _))
  (return false))

(fn Thinking
  (return false))