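; BP_Butler is an interactable butler NPC that talks to the VR player through a child-actor speech bubble.
; Every tick the bubble yaws toward the player camera, clamped to a narrow arc and offset by the mesh yaw captured at BeginPlay.
; Interact plays a formal bow and returns a "Talk" option box, whose activation speaks the current Conversation line.
; Converse always speaks the first line, and Thinking is a stub returning false.
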(event EventBeginPlay
  (Variables|Default|SetRotationOffset (- -9e+01 (.yaw (Transformation|GetWorldRotation (Variables|Character|GetMesh))))))

(event EventActorBeginOverlap
  (params (OtherActor :type Actor%20Object%20Reference)))

(event EventTick
  (params (DeltaSeconds :type Float%20%28single-precision%29))
  (bind _location (CallFunction|GetPlayerVRCameraProperties))
  (Transformation|SetRelativeRotation (Variables|Default|GetSpeechBubble) (Math|Rotator|MakeRotator 0.0 0.0 (Math|Float|ClampAngle (+ (.yaw (Math|Rotator|FindLookatRotation (Transformation|GetWorldLocation (Variables|Default|GetSpeechBubble)) _location)) (Variables|Default|GetRotationOffset)) -3e+01 3e+01)) false false))

(fn ConstructionScript)

(fn Converse
  (bind _asbp_speech_bubble (Utilities|Casting|CastToBP_SpeechBubble (Variables|/Script/Engine.ChildActorComponent|GetChildActor (Variables|Default|GetSpeechBubble)))
    (:then
      (Default|Speak _asbp_speech_bubble (Utilities|Array|Get(acopy) (Variables|Default|GetConversation))))
    (:CastFailed
      _))
  (return))

(fn ActivateOption
  (CallFunction|Talk (Variables|Default|GetConvoIndex))
  (return 0))

(fn Interact
  (Components|Animation|PlayAnimation (Variables|Character|GetMesh) "/Game/VengeanceRising/Commons/Characters/Butler/quick_formal_bow.quick_formal_bow" false)
  (return true "-30.000000,30.000000,80.000000" "Talk"))

(fn Talk
  (params (Index :type Integer))
  (bind _asbp_speech_bubble (Utilities|Casting|CastToBP_SpeechBubble (Variables|/Script/Engine.ChildActorComponent|GetChildActor (Variables|Default|GetSpeechBubble)))
    (:then
      (Default|Speak _asbp_speech_bubble (Utilities|Array|Get(acopy) (Variables|Default|GetConversation) Index)))
    (:CastFailed
      _))
  (return false))

(fn Thinking
  (return false))