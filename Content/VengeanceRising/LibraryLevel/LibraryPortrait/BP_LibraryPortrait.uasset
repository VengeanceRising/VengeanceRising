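; Interactable library portrait that can send the player to another level or serve as a source of inspection thoughts.
; Interacting offers an "Inspect" option; activating it in puzzle mode saves the player's transform, fades to black, plays harp music and opens NextLevel after an audio delay.
; Otherwise activation switches the thought index, and Thinking shows that thought as a subtitle through BP_DiningHallPlayer.
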(event Custom|Go
  (params (Level :type Name))
  (Utilities|FlowControl|Delay (Variables|Default|GetAudioDelay))
  (Game|OpenLevel(byName) Level))

(event EventBeginPlay
  (bind _outactors (Actor|GetAllActorsOfClass "/Game/VengeanceRising/DiningHallLevel/BP_DiningHallPlayer.BP_DiningHallPlayer_C"))
  (Variables|Default|SetPlayer (Utilities|Array|Get(acopy) _outactors)))

(event Collision|EventActorBeginOverlap
  (params (OtherActor :type Actor%20Object%20Reference)))

(event EventTick
  (params (DeltaSeconds :type Float%20%28single-precision%29)))

(fn ConstructionScript)

(fn ActivateOption
  (bind _nextlevel (Variables|Default|GetNextLevel))
  (bind _player (Variables|Default|GetPlayer))
  (if (Variables|Default|GetGoToPuzzle)
    (if (Utilities|Name|Equal(Name) _nextlevel "None")
      _
      (else
        (Default|UpdatePlayerTransform _player)
        (Default|FadetoBlack _player)
        (Audio|PlaySoundatLocation "/Game/VengeanceRising/Commons/Sounds/My_lady_careys_dompe_-_harp.My_lady_careys_dompe_-_harp" (Transformation|GetWorldLocation (Variables|Default|GetStaticMesh)))
        (CallFunction|Go _nextlevel)))
    (else
      (Variables|Default|SetThoughtIndex 1)))
  (return 0))

(fn Interact
  (return true (Variables|Default|GetSpawnOffset) "Inspect"))

(fn Talk
  (params (Index :type Integer))
  (return false))

(fn Thinking
  (bind _asbp_dining_hall_player (Utilities|Casting|CastToBP_DiningHallPlayer (Game|Player|GetPlayerPawn 0))
    (:then
      (Default|DisplaySubtitles _asbp_dining_hall_player (Utilities|Array|Get(acopy) (Variables|Default|GetThoughts) (Variables|Default|GetThoughtIndex))))
    (:CastFailed
      _))
  (return false))