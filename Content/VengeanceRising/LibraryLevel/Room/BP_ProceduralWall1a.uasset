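; BP_ProceduralWall1a is a procedural wall actor for the library level that builds a straight run of segments toward an EndPoint offset.
; The construction script ignores height and yaws the BaseFloor component to face EndPoint, with a -90 degree correction so local Y follows the run.
; It then adds static mesh components under BaseFloor at WallWidth intervals, rounding the count up to cover the distance.
; The event graph is empty.
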(event EventBeginPlay)

(event Collision|EventActorBeginOverlap
  (params (OtherActor :type Actor%20Object%20Reference)))

(event EventTick
  (params (DeltaSeconds :type Float%20%28single-precision%29)))

(fn ConstructionScript
  (bind _returnvalue (Transformation|GetActorLocation))
  (if (Math|Vector|NotEqual(Vector) (* (Variables|Default|GetEndPoint) "1.000000,1.000000, 0") "0, 0, 0" 0.0001)
    ;[1 1 1] Use only if neccesary to enforce orientation
    (Transformation|SetWorldRotation (Variables|Default|GetBaseFloor) (Math|Rotator|MakeRotator 0.0 0.0 (+ (.Yaw (Math|Rotator|BreakRotator (Math|Rotator|FindLookatRotation _returnvalue (+ (* _returnvalue "1.000000,1.000000, 0") (* (Variables|Default|GetEndPoint) "1.000000,1.000000, 0"))))) -9e+01)) false false)
    (for _index (range 1 (- (Math|Float|Ceil (/ (Math|Vector|VectorLength (* (Variables|Default|GetEndPoint) "1.000000,1.000000, 0")) (Variables|Default|GetWallWidth))) 1))
      (bind _returnvalue_2 (AddComponent|AddStaticMeshComponent false))
      (Class|SceneComponent|Attachto _returnvalue_2 (Variables|Default|GetBaseFloor) "None" "KeepRelativeOffset" true)
      (Transformation|SetRelativeLocation _returnvalue_2 (Math|Vector|MakeVector 0.0 (* _index (Variables|Default|GetWallWidth)) 0.0) false false))))