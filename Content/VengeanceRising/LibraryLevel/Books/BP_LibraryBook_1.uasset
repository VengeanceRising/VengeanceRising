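; BP_LibraryBook_1 is a configurable book prop for the library level, set up entirely in its construction script.
; It adds one identity-transform instance to each of two book instance components, then BookOption1 chooses which one is visible.
; BookOption2 switches both between two book material instances, on a different element index for each component.
; An unconnected random-color dynamic material branch never runs, and the event graph is empty apart from disabled stubs.
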(event EventBeginPlay)

(event Collision|EventActorBeginOverlap
  (params (OtherActor :type Actor%20Object%20Reference)))

(event EventTick
  (params (DeltaSeconds :type Float%20%28single-precision%29)))

(fn ConstructionScript
  (bind _returnvalue (Math|Transform|MakeTransform "0, 0, 0"))
  (bind _book_option_1 (Variables|Settings|GetBook%20Option%201))
  (bind _book1_instance (Variables|Default|GetBook1_Instance))
  (bind _book2_instance (Variables|Default|GetBook2_Instance))
  (Components|InstancedStaticMesh|AddInstance (Variables|Default|GetBook1_Instance) _returnvalue)
  (Components|InstancedStaticMesh|AddInstance (Variables|Default|GetBook2_Instance) _returnvalue)
  (Rendering|SetVisibility (Variables|Default|GetBook1_Instance) _book_option_1 false)
  (Rendering|SetVisibility (Variables|Default|GetBook2_Instance) (not _book_option_1) false)
  ;[1 1 1] Material Selection
  (if (Variables|Settings|GetBook%20Option%202)
    (Rendering|Material|SetMaterial _book2_instance 5 "/Game/VengeanceRising/LibraryLevel/ImportedFromFreeLibrary/Books/Materials/MI_book1_a.MI_book1_a")
    (Rendering|Material|SetMaterial _book1_instance 0 "/Game/VengeanceRising/LibraryLevel/ImportedFromFreeLibrary/Books/Materials/MI_book1_a.MI_book1_a")
    (else
      (Rendering|Material|SetMaterial _book2_instance 5 "/Game/VengeanceRising/LibraryLevel/ImportedFromFreeLibrary/Books/Materials/MI_book1_b.MI_book1_b")
      (Rendering|Material|SetMaterial _book1_instance 0 "/Game/VengeanceRising/LibraryLevel/ImportedFromFreeLibrary/Books/Materials/MI_book1_b.MI_book1_b"))))