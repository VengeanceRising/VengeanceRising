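; BP_LibraryDoor is an interactable library door that takes the player to another level.
; Interact returns an "Open" prompt box with an offset, and Thinking shows a thought as a subtitle on the player pawn.
; ActivateOption, when NextLevel is set, fades the BP_DiningHallPlayer cached at BeginPlay to black, plays a sound at the mesh, then opens that level after a short delay.
; Talk is a stub returning false.
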(event Custom|Go
  (params (Level :type Name))
  (Utilities|FlowControl|Delay 1.0)
  (Game|OpenLevel(byName) Level))

(event EventBeginPlay
  (bind _outactors (Actor|GetAllActorsOfClass "/Game/VengeanceRising/DiningHallLevel/BP_DiningHallPlayer.BP_DiningHallPlayer_C"))
  (Variables|Default|SetPlayer (Utilities|Array|Get(acopy) _outactors)))

(event Collision|EventActorBeginOverlap
  (params (OtherActor :type Actor%20Object%20Reference)))

(event EventTick
  (params (DeltaSeconds :type Float%20%28single-precision%29)))

(fn ConstructionScript)

(fn ActivateOption
  (bind _nextlevel (Variables|Default|GetNextLevel))
  (if (Utilities|Name|Equal(Name) _nextlevel "None")
    _
    (else
      (Default|FadetoBlack (Variables|Default|GetPlayer))
      (Audio|PlaySoundatLocation "/Game/VengeanceRising/Commons/Sounds/146173__d-w__chair-dining-chair-wooden-person-sit-01.146173__d-w__chair-dining-chair-wooden-person-sit-01" (Transformation|GetWorldLocation (Variables|Default|GetStaticMesh)))
      (CallFunction|Go _nextlevel)))
  (return 0))

(fn Interact
  (return true (Variables|Default|GetSpawnOffset) "Open"))

(fn Talk
  (params (Index :type Integer))
  (return false))

(fn Thinking
  (bind _asbp_dining_hall_player (Utilities|Casting|CastToBP_DiningHallPlayer (Game|Player|GetPlayerPawn 0))
    (:then
      (Default|DisplaySubtitles _asbp_dining_hall_player (Utilities|Array|Get(acopy) (Variables|Default|GetThoughts) (Variables|Default|GetThoughtIndex))))
    (:CastFailed
      _))
  (return false))