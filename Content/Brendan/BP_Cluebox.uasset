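; BP_Cluebox is a clue box actor that displays a picture and has a color cube that can cycle through five colors.
; The construction script applies the Picture material to Screenshot and creates a dynamic material instance for ColorCube.
; Each SwitchColor call steps a MultiGate to set that instance's Color parameter, resetting after the last color.
; The Clickable function is empty.
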(event Custom|SwitchColor
  (bind _dmi (Variables|Default|GetDMI))
  (Utilities|FlowControl|MultiGate false false 0 :!label _label
    (:Out%200
      (Rendering|Material|SetVectorParameterValue _dmi "Color" "(R=0.092262,G=0.301557,B=0.905000,A=1.000000)" :!class /Script/Engine.MaterialInstanceDynamic))
    (:Out%201
      (Rendering|Material|SetVectorParameterValue _dmi "Color" "(R=0.875000,G=0.809016,B=0.183750,A=1.000000)" :!class /Script/Engine.MaterialInstanceDynamic))
    (:Out%202
      (Rendering|Material|SetVectorParameterValue _dmi "Color" "(R=1.000000,G=0.210000,B=0.949128,A=1.000000)" :!class /Script/Engine.MaterialInstanceDynamic))
    (:Out%203
      (Rendering|Material|SetVectorParameterValue _dmi "Color" "(R=0.323529,G=0.850000,B=0.238000,A=1.000000)" :!class /Script/Engine.MaterialInstanceDynamic))
    (:Out%204
      (Rendering|Material|SetVectorParameterValue _dmi "Color" "(R=0.870000,G=0.472708,B=0.187050,A=1.000000)" :!class /Script/Engine.MaterialInstanceDynamic)
      (goto _label Reset))))

(event EventBeginPlay)

(event EventActorBeginOverlap
  (params (OtherActor :type Actor%20Object%20Reference)))

(event EventTick
  (params (DeltaSeconds :type Float%20%28single-precision%29)))

(fn ConstructionScript
  (Rendering|Material|SetMaterial (Variables|Default|GetScreenshot) 0 (Variables|Default|GetPicture))
  (bind _returnvalue (Rendering|Material|CreateDynamicMaterialInstance (Variables|Default|GetColorCube) 0 "/Game/Brendan/M_Color.M_Color" :!class /Script/Engine.PrimitiveComponent))
  (Variables|Default|SetDMI _returnvalue))

(fn Clickable
  (return))