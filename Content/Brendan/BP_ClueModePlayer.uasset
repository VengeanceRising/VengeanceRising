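; Player for clue mode, a clue board where clue boxes are inspected, dragged and combined, with a tightly clamped camera view.
; Tick traces through a mouse cursor component to set the hovered clue or close button and tint the cursor.
; Left click uses a delayed count to recolor or expand details, while right click drags via a physics handle.
; Events spawn stored clues, randomly placing unpositioned ones, and replace valid pairs with their combined result.
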(event Custom|CombineClues
  (params (FirstClue :type BP%20Cluebox%20Object%20Reference) (SecondClue :type BP%20Cluebox%20Object%20Reference))
  (bind _name (Variables|/Game/Brendan/BP_Cluebox.BP_Cluebox_C|GetName FirstClue))
  (bind _name_2 (Variables|/Game/Brendan/BP_Cluebox.BP_Cluebox_C|GetName SecondClue))
  ;[1 1 1] Clue Combinations
  (bind _array_element (Utilities|Array|ForEachLoopwithBreak (Variables|Default|GetClueCombi) :!label _label)
    (:LoopBody
      (if (or (and (Utilities|Enum|Equal(Enum) (.FirstClue (Utilities|Struct|BreakBPS_ClueCombi _array_element)) _name) (Utilities|Enum|Equal(Enum) (.SecondClue (Utilities|Struct|BreakBPS_ClueCombi _array_element)) _name_2)) (and (Utilities|Enum|Equal(Enum) (.FirstClue (Utilities|Struct|BreakBPS_ClueCombi _array_element)) _name_2) (Utilities|Enum|Equal(Enum) (.SecondClue (Utilities|Struct|BreakBPS_ClueCombi _array_element)) _name)))
        (Variables|Default|SetcanCombine true)
        (goto _label Break)))
    (:Completed
      (if (Variables|Default|GetcanCombine)
        (Effects|SpawnEmitteratLocation "/Game/VengeanceRising/LibraryLevel/ImportedFromFreeLibrary/StarterContent/Particles/P_Steam_Lit.P_Steam_Lit" (Transformation|GetActorLocation FirstClue))
        (Actor|DestroyActor FirstClue)
        (Actor|DestroyActor SecondClue)
        (CallFunction|SpawnClue (.ResultClue (Utilities|Struct|BreakBPS_ClueCombi _array_element)))
        (else
          (Development|PrintString "Cannot Combine!"))))))

(event Custom|SpawnMyClues
  ;[1 1 1] Spawn all of "MyClues"
  (for _array_element (Variables|Default|GetMyClues)
    (if (Math|Vector|Equal(Vector) (.Location (Utilities|Struct|BreakBPS_Clue _array_element)) "0, 0, 0" 0.0001)
      (CallFunction|SpawnClue (Utilities|Struct|MakeBPS_Clue (.Name (Utilities|Struct|BreakBPS_Clue _array_element)) (.LongDescription (Utilities|Struct|BreakBPS_Clue _array_element)) (.Thumbnail (Utilities|Struct|BreakBPS_Clue _array_element)) (Math|Vector|MakeVector 641.0 (Math|Random|RandomFloatinRange -5.6e+02 5.8e+02) (Math|Random|RandomFloatinRange -2e+02 6e+02)) (.ColorIndex (Utilities|Struct|BreakBPS_Clue _array_element))))
      (else
        (CallFunction|SpawnClue _array_element)))))

(event Custom|DoubleClick
  (bind _targetclue (Variables|Default|GetTargetClue))
  ;[1 1 1] Open details pane for clues
  (Default|CallExpandonClick (Variables|/Game/Brendan/BP_ExpandedClue.BP_ExpandedClue_C|GetExClue (Variables|Default|Get3DWidget)) (Variables|/Game/Brendan/BP_Cluebox.BP_Cluebox_C|GetLong%20Description _targetclue) (Variables|/Game/Brendan/BP_Cluebox.BP_Cluebox_C|GetName _targetclue) (Variables|/Game/Brendan/BP_Cluebox.BP_Cluebox_C|GetThumbnail _targetclue)))

(event Custom|SpawnClue
  (params (Clue :type BPS%20Clue%20Structure))
  (bind (_name _longdescription _thumbnail _location _colorindex) (Utilities|Struct|BreakBPS_Clue Clue))
  ;[1 1 1] Spawn a cluebox
  (bind _returnvalue (Game|SpawnActorfromClass "/Game/Brendan/BP_Cluebox.BP_Cluebox_C" (Math|Transform|MakeTransform _location "0, 0, 0" "1,1,1") "AdjustIfPossibleButAlwaysSpawn" 0 0))
  (Variables|/Game/Brendan/BP_Cluebox.BP_Cluebox_C|SetName _returnvalue _name)
  (Variables|/Game/Brendan/BP_Cluebox.BP_Cluebox_C|SetLong%20Description _returnvalue _longdescription)
  (Variables|/Game/Brendan/BP_Cluebox.BP_Cluebox_C|SetThumbnail _returnvalue _thumbnail)
  (Variables|/Game/Brendan/BP_Cluebox.BP_Cluebox_C|SetToggleColor _returnvalue _colorindex))

(event EventBeginPlay
  (bind _returnvalue (Game|GetPlayerCameraManager 0))
  ;[1 1 1] Setting max turn radius
  (Variables|/Script/Engine.PlayerCameraManager|SetViewPitchMin _returnvalue -2e+01)
  (Variables|/Script/Engine.PlayerCameraManager|SetViewPitchMax _returnvalue 2e+01)
  (Variables|/Script/Engine.PlayerCameraManager|SetViewYawMin _returnvalue -2e+01)
  (Variables|/Script/Engine.PlayerCameraManager|SetViewYawMax _returnvalue 2e+01))

(event EventTick
  (params (DeltaSeconds :type Float%20%28single-precision%29))
  (bind _returnvalue (Game|GetPlayerController 0))
  (bind _3dwidget (Variables|Default|Get3DWidget))
  (bind _bpc_mousecursor (Variables|Default|GetBPC_MouseCursor))
  (bind (_deltax _deltay) (Class|PlayerController|GetInputMouseDelta _returnvalue))
  ;[1 1 1] Mouse Cursor and its onHit events
  (bind _tracehit (Default|Update (Variables|Default|GetBPC_MouseCursor) _deltax _deltay "0, 0, 0"))
  (bind _asbp_cluebox (Utilities|Casting|CastToBP_Cluebox (.HitActor (Collision|BreakHitResult _tracehit)))
    (:then
      (Variables|Default|SetHeldClue (.HitComponent (Collision|BreakHitResult _tracehit)))
      (Physics|Components|PhysicsHandle|SetTargetLocation (Variables|Default|GetPhysicsHandle) (Default|GetCursorLocation (Variables|Default|GetBPC_MouseCursor)))
      (Default|SetCursorColor _bpc_mousecursor "(R=0.000000,G=0.000000,B=1.000000,A=0.500000)")
      (Variables|Default|SetonClue true)
      (Variables|Default|SetTargetClue _asbp_cluebox))
    (:CastFailed
      (if (and (== (.HitComponent (Collision|BreakHitResult _tracehit)) (Variables|/Game/Brendan/BP_ExpandedClue.BP_ExpandedClue_C|GetCloseButton _3dwidget)) (Variables|/Game/Brendan/BPW_ExpandedClue.BPW_ExpandedClue_C|GetisActive (Variables|/Game/Brendan/BP_ExpandedClue.BP_ExpandedClue_C|GetExClue _3dwidget)))
        (Default|SetCursorColor _bpc_mousecursor "(R=1.000000,G=0.000000,B=0.008924,A=1.000000)")
        (Variables|Default|SetonClose true)
        (else
          (Default|SetCursorColor _bpc_mousecursor "(R=1.000000,G=1.000000,B=1.000000,A=1.000000)")
          (Variables|Default|SetonClue false)
          (Variables|Default|SetonClose false))))))

(event Input|ActionEvents|InputActionLeftClick
  (params (Key :type Key%20Structure :default "AnyKey"))
  ;[1 1 1] Double Click on ClueBox
  (:Pressed
    (if (Variables|Default|GetonClue)
      (Math|Integer|IncrementInt (Variables|Default|GetClickCount)
        (:%20%20
          (bind _output_get (Variables|Default|SetTargetForAction (Variables|Default|GetTargetClue)))
          (Utilities|FlowControl|Delay 0.5)
          (if (== (Variables|Default|GetClickCount) 1)
            (Variables|Default|SetClickCount 0)
            (Default|SwitchColor _output_get)
            (elif (> (Variables|Default|GetClickCount) 1)
              (CallFunction|DoubleClick)
              (Variables|Default|SetClickCount 0)))))
      (elif (Variables|Default|GetonClose)
        (Default|CloseWidget (Variables|/Game/Brendan/BP_ExpandedClue.BP_ExpandedClue_C|GetExClue (Variables|Default|Get3DWidget)))))))

(event Input|ActionEvents|InputActionRightClick
  (params (Key :type Key%20Structure :default "AnyKey"))
  ;[1 1 1] Dragging clues around
  (:Pressed
    (if (Variables|Default|GetonClue)
      (Class|PhysicsHandleComponent|GrabComponent (Variables|Default|GetPhysicsHandle) (Variables|Default|GetHeldClue) "None" (Transformation|GetWorldLocation (Variables|Default|GetHeldClue)) false)))
  (:Released
    (Physics|Components|PhysicsHandle|ReleaseComponent (Variables|Default|GetPhysicsHandle))))

(event Input|AxisEvents|InputAxisLookUpRate
  (params (AxisValue :type Float%20%28single-precision%29))
  ;[1 1 1] Rotating View
  (Pawn|Input|AddControllerPitchInput (* AxisValue (Variables|Default|GetBaseLookUpRate) (Utilities|Time|GetWorldDeltaSeconds))))

(event Input|AxisEvents|InputAxisTurnRate
  (params (AxisValue :type Float%20%28single-precision%29))
  ;[1 1 1] Rotating View
  (Pawn|Input|AddControllerYawInput (* AxisValue (Variables|Default|GetBaseTurnRate) (Utilities|Time|GetWorldDeltaSeconds))))

(event Input|AxisEvents|InputAxisTurn
  (params (AxisValue :type Float%20%28single-precision%29))
  ;[1 1 1] Rotating View
  (Pawn|Input|AddControllerYawInput (/ AxisValue 5.0)))

(event Input|AxisEvents|InputAxisLookUp
  (params (AxisValue :type Float%20%28single-precision%29))
  ;[1 1 1] Rotating View
  (Pawn|Input|AddControllerPitchInput (/ AxisValue 5.0)))

(fn ConstructionScript)