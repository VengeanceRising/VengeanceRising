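; BP_InventoryPlayer is a player Blueprint for interacting with a 3D inventory widget using a mouse-driven cursor and a narrowly clamped camera view.
; Each Tick, BPCMouseCursor updates from mouse delta, moves the PhysicsHandle target, and passes its trace hit to HitTarget.
; HitTarget recolors the cursor and flags whether it is over the slider, item or close button.
; Left click toggles the pane or grabs the hovered slider or item, and release drops it.
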(event Custom|HitTarget
  (params (Hit%20component :type Primitive%20Component%20Object%20Reference))
  (bind _bpc_mousecursor (Variables|Default|GetBPC_MouseCursor))
  (bind _3dwidget (Variables|Default|Get3DWidget))
  ;[1 1 1] Setting the click target
  (if (== Hit%20component (Variables|/Game/Brendan/BP_ItemDetails.BP_ItemDetails_C|GetSlider _3dwidget))
    (Default|SetCursorColor _bpc_mousecursor "(R=0.000000,G=0.000000,B=1.000000,A=1.000000)")
    (Variables|Default|SetonSlider true)
    (Variables|Default|SetHeldComponent Hit%20component :!label _label)
    (elif (== Hit%20component (Variables|/Game/Brendan/BP_ItemDetails.BP_ItemDetails_C|GetItem _3dwidget))
      (Default|SetCursorColor _bpc_mousecursor "(R=0.000000,G=0.000000,B=1.000000,A=1.000000)")
      (Variables|Default|SetonItem true)
      (goto _label)
      (elif (== Hit%20component (Variables|/Game/Brendan/BP_ItemDetails.BP_ItemDetails_C|GetCloseButton _3dwidget))
        (Default|SetCursorColor _bpc_mousecursor "(R=1.000000,G=0.000000,B=0.011861,A=1.000000)")
        (Variables|Default|SetonClose true)
        (else
          (Default|SetCursorColor _bpc_mousecursor "(R=1.000000,G=1.000000,B=1.000000,A=1.000000)")
          (Variables|Default|SetonClose false)
          (Variables|Default|SetonItem false)
          (Variables|Default|SetonSlider false)
          (Variables|Default|SetHeldComponent 0)
          (Physics|Components|PhysicsHandle|ReleaseComponent (Variables|Default|GetPhysicsHandle)))))))

(event EventBeginPlay
  (bind _returnvalue (Game|GetPlayerCameraManager 0))
  ;[1 1 1] Setting max turn radius
  (Variables|/Script/Engine.PlayerCameraManager|SetViewPitchMin _returnvalue -2e+01)
  (Variables|/Script/Engine.PlayerCameraManager|SetViewPitchMax _returnvalue 2e+01)
  (Variables|/Script/Engine.PlayerCameraManager|SetViewYawMin _returnvalue -2e+01)
  (Variables|/Script/Engine.PlayerCameraManager|SetViewYawMax _returnvalue 2e+01))

(event EventTick
  (params (DeltaSeconds :type Float%20%28single-precision%29))
  (bind _returnvalue (Game|GetPlayerController 0))
  (bind _bpc_mousecursor (Variables|Default|GetBPC_MouseCursor))
  (bind (_deltax _deltay) (Class|PlayerController|GetInputMouseDelta _returnvalue))
  ;[1 1 1] Mouse Cursor and its onHit events
  (bind _tracehit (Default|Update _bpc_mousecursor _deltax _deltay "0,0.000000, 0"))
  (Physics|Components|PhysicsHandle|SetTargetLocation (Variables|Default|GetPhysicsHandle) (Default|GetCursorLocation _bpc_mousecursor))
  (CallFunction|HitTarget (.HitComponent (Collision|BreakHitResult _tracehit))))

(event Input|ActionEvents|InputActionLeftClick
  (params (Key :type Key%20Structure :default "AnyKey"))
  (bind _physicshandle (Variables|Default|GetPhysicsHandle))
  (bind _heldcomponent (Variables|Default|GetHeldComponent))
  (:Pressed
    (if (Variables|Default|GetonClose)
      (Default|TogglePane (Variables|Default|Get3DWidget))
      (elif (Variables|Default|GetonItem)
        (Class|PhysicsHandleComponent|GrabComponent _physicshandle _heldcomponent "None" (Transformation|GetWorldLocation _heldcomponent) false :!label _label)
        (elif (Variables|Default|GetonSlider)
          (goto _label)))))
  (:Released
    (Physics|Components|PhysicsHandle|ReleaseComponent _physicshandle)))

(event Input|AxisEvents|InputAxisLookUpRate
  (params (AxisValue :type Float%20%28single-precision%29))
  ;[1 1 1] Rotating View
  (Pawn|Input|AddControllerPitchInput (* AxisValue (Variables|Default|GetBaseLookUpRate) (Utilities|Time|GetWorldDeltaSeconds))))

(event Input|AxisEvents|InputAxisTurnRate
  (params (AxisValue :type Float%20%28single-precision%29))
  ;[1 1 1] Rotating View
  (Pawn|Input|AddControllerYawInput (* AxisValue (Variables|Default|GetBaseTurnRate) (Utilities|Time|GetWorldDeltaSeconds))))

(event Input|AxisEvents|InputAxisTurn
  (params (AxisValue :type Float%20%28single-precision%29))
  ;[1 1 1] Rotating View
  (Pawn|Input|AddControllerYawInput (/ AxisValue 5.0)))

(event Input|AxisEvents|InputAxisLookUp
  (params (AxisValue :type Float%20%28single-precision%29))
  ;[1 1 1] Rotating View
  (Pawn|Input|AddControllerPitchInput (/ AxisValue 5.0)))

(fn ConstructionScript)