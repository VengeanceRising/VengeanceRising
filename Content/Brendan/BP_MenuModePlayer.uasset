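; Player for a menu mode where the user looks around within clamped angles and works with clue boxes.
; Each tick, a mouse cursor component traces, tints the cursor and flags whether a clue or the widget's close button is hovered.
; Right-click drags clues through a physics handle.
; Left-click uses a delayed click counter: single switches clue color, double expands its details in a 3D widget, and clicking close dismisses it.
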(event Custom|DoubleClick
  (bind _targetclue (Variables|Default|GetTargetClue))
  (Default|CallExpandonClick (Variables|/Game/Brendan/BP_ExpandedClue.BP_ExpandedClue_C|GetExClue (Variables|Default|Get3DWidget)) (Variables|/Game/Brendan/BP_Cluebox.BP_Cluebox_C|GetLong%20Description _targetclue) (Variables|/Game/Brendan/BP_Cluebox.BP_Cluebox_C|GetCharateristics _targetclue) (Variables|/Game/Brendan/BP_Cluebox.BP_Cluebox_C|GetPic _targetclue)))

(event EventBeginPlay)

(event EventActorBeginOverlap
  (params (OtherActor :type Actor%20Object%20Reference)))

(event EventBeginPlay
  (bind _returnvalue (Game|GetPlayerCameraManager 0))
  (Variables|/Script/Engine.PlayerCameraManager|SetViewPitchMin _returnvalue -9e+01)
  (Variables|/Script/Engine.PlayerCameraManager|SetViewPitchMax _returnvalue 9e+01)
  (Variables|/Script/Engine.PlayerCameraManager|SetViewYawMin _returnvalue -9e+01)
  (Variables|/Script/Engine.PlayerCameraManager|SetViewYawMax _returnvalue 9e+01))

(event EventTick
  (params (DeltaSeconds :type Float%20%28single-precision%29)))

(event EventTick
  (params (DeltaSeconds :type Float%20%28single-precision%29))
  (bind _returnvalue (Game|GetPlayerController 0))
  (bind _3dwidget (Variables|Default|Get3DWidget))
  (bind _bpc_mousecursor (Variables|Default|GetBPC_MouseCursor))
  (bind (_deltax _deltay) (Class|PlayerController|GetInputMouseDelta _returnvalue))
  (bind _tracehit (Default|Update (Variables|Default|GetBPC_MouseCursor) _deltax _deltay "0, 0, 0"))
  (bind _asbp_cluebox (Utilities|Casting|CastToBP_Cluebox (.HitActor (Collision|BreakHitResult _tracehit)))
    (:then
      (Variables|Default|SetHeldClue (.HitComponent (Collision|BreakHitResult _tracehit)))
      (if (Variables|Default|GetisPressed)
        (Physics|Components|PhysicsHandle|SetTargetLocation (Variables|Default|GetPhysicsHandle) (Default|GetCursorLocation (Variables|Default|GetBPC_MouseCursor))))
      (Default|SetCursorColor _bpc_mousecursor "(R=0.000000,G=0.000000,B=1.000000,A=0.500000)")
      (Variables|Default|SetonClue true)
      (Variables|Default|SetTargetClue _asbp_cluebox))
    (:CastFailed
      (if (and (== (.HitComponent (Collision|BreakHitResult _tracehit)) (Variables|/Game/Brendan/BP_ExpandedClue.BP_ExpandedClue_C|GetCloseButton _3dwidget)) (Variables|/Game/Brendan/BPW_ExpandedClue.BPW_ExpandedClue_C|GetisActive (Variables|/Game/Brendan/BP_ExpandedClue.BP_ExpandedClue_C|GetExClue _3dwidget)))
        (Default|SetCursorColor _bpc_mousecursor "(R=1.000000,G=0.000000,B=0.008924,A=1.000000)")
        (Variables|Default|SetonClose true)
        (else
          (Default|SetCursorColor _bpc_mousecursor "(R=1.000000,G=1.000000,B=1.000000,A=1.000000)")
          (Variables|Default|SetonClue false)
          (Variables|Default|SetonClose false))))))

(event Input|ActionEvents|InputActionLeftClick
  (params (Key :type Key%20Structure :default "AnyKey"))
  ;[1 1 1] Double Click on ClueBox
  (:Pressed
    (if (Variables|Default|GetonClue)
      (Math|Integer|IncrementInt (Variables|Default|GetClickCount)
        (:%20%20
          (bind _output_get (Variables|Default|SetTargetForAction (Variables|Default|GetTargetClue)))
          (Utilities|FlowControl|Delay 0.5)
          (if (== (Variables|Default|GetClickCount) 1)
            (Variables|Default|SetClickCount 0)
            (Default|SwitchColor _output_get)
            (elif (> (Variables|Default|GetClickCount) 1)
              (CallFunction|DoubleClick)
              (Variables|Default|SetClickCount 0)))))
      (elif (Variables|Default|GetonClose)
        (Default|CloseWidget (Variables|/Game/Brendan/BP_ExpandedClue.BP_ExpandedClue_C|GetExClue (Variables|Default|Get3DWidget)))))))

(event Input|ActionEvents|InputActionRightClick
  (params (Key :type Key%20Structure :default "AnyKey"))
  (bind _heldclue (Variables|Default|GetHeldClue))
  (bind _returnvalue (Transformation|GetWorldLocation _heldclue))
  (:Pressed
    (Variables|Default|SetisPressed true)
    (if (Variables|Default|GetonClue)
      (Class|PhysicsHandleComponent|GrabComponent (Variables|Default|GetPhysicsHandle) (Variables|Default|GetHeldClue) "None" (Math|Vector|MakeVector (.x _returnvalue) (.y _returnvalue) (.z _returnvalue)) false)))
  (:Released
    (Variables|Default|SetisPressed false)
    (Physics|Components|PhysicsHandle|ReleaseComponent (Variables|Default|GetPhysicsHandle))))

(event Input|AxisEvents|InputAxisLookUpRate
  (params (AxisValue :type Float%20%28single-precision%29))
  ;[1 1 1] Rotating View
  (Pawn|Input|AddControllerPitchInput (* AxisValue (Variables|Default|GetBaseLookUpRate) (Utilities|Time|GetWorldDeltaSeconds))))

(event Input|AxisEvents|InputAxisTurnRate
  (params (AxisValue :type Float%20%28single-precision%29))
  ;[1 1 1] Rotating View
  (Pawn|Input|AddControllerYawInput (* AxisValue (Variables|Default|GetBaseTurnRate) (Utilities|Time|GetWorldDeltaSeconds))))

(event Input|AxisEvents|InputAxisTurn
  (params (AxisValue :type Float%20%28single-precision%29))
  ;[1 1 1] Rotating View
  (Pawn|Input|AddControllerYawInput (/ AxisValue 5.0)))

(event Input|AxisEvents|InputAxisLookUp
  (params (AxisValue :type Float%20%28single-precision%29))
  ;[1 1 1] Rotating View
  (Pawn|Input|AddControllerPitchInput (/ AxisValue 5.0)))

(fn ConstructionScript)