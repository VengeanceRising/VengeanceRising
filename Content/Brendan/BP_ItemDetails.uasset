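; BP_ItemDetails is an item details pane actor combining an item, a slider and a BPW_ItemDetails widget.
; On BeginPlay it caches the widget and records the slider's world height as zero.
; Each tick it turns the slider's vertical offset from that height into a percentage of a fixed travel distance, which is only printed.
; TogglePane flips the active flag, toggles slider and item visibility, and always calls CloseWidget on the widget.
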(event Custom|TogglePane
  (Variables|Default|SetisActive (not (Variables|Default|GetisActive)))
  (Rendering|ToggleVisibility (Variables|Default|GetSlider) false)
  (Rendering|ToggleVisibility (Variables|Default|GetItem) false)
  (Default|CloseWidget (Variables|Default|GetItemD)))

(event EventBeginPlay
  (bind _asbpw_item_details (Utilities|Casting|CastToBPW_ItemDetails (UserInterface|GetUserWidgetObject (Variables|Default|GetItemDetails))))
  (Variables|Default|SetItemD _asbpw_item_details)
  (Variables|Default|SetZeroing (.z (Transformation|GetWorldLocation (Variables|Default|GetSlider)))))

(event Collision|EventActorBeginOverlap
  (params (OtherActor :type Actor%20Object%20Reference)))

(event EventTick
  (params (DeltaSeconds :type Float%20%28single-precision%29))
  (bind _output_get (Variables|Default|SetScaleVal (* (/ (- (.z (Transformation|GetWorldLocation (Variables|Default|GetSlider))) (Variables|Default|GetZeroing)) 147.0) 1e+02)))
  (Development|PrintString (Utilities|String|ToString(Float) _output_get)))

(fn ConstructionScript)